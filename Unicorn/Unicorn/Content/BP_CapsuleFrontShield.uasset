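; BP_CapsuleFrontShield is a spell actor: a front shield that can also act as a ram against whatever it touches.
; Activation toggles mesh visibility and the query-only RamCollider, while SetRamming recolors the shield through a dynamic material instance.
; While ramming, overlaps or hits on pawns other than its parent actor apply knockback, stun and damage via messages.
; Dispatchers report static mesh and pawn impacts back to listeners.
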(event `self.ReceiveBeginPlay`
  (`parent.ReceiveBeginPlay`))

(event `self.ActivateSpell`
  (`parent.ActivateSpell`)
  (`SceneComponent.SetVisibility` (`self.Mesh`) true false)
  (`PrimitiveComponent.SetCollisionEnabled` (`self.RamCollider`) "QueryOnly"))

(event `self.DeactivateSpell`
  (`parent.DeactivateSpell`)
  (`SceneComponent.SetVisibility` (`self.Mesh`) false false)
  (`PrimitiveComponent.SetCollisionEnabled` (`self.RamCollider`) "NoCollision")
  (`self.SetRamming` false))

(event `self.RamCollider.OnComponentBeginOverlap`
  (params (OverlappedComponent :type "PrimitiveComponent Object Reference") (OtherActor :type "Actor Object Reference") (OtherComp :type "PrimitiveComponent Object Reference") (OtherBodyIndex :type Integer) (bFromSweep :type Boolean) (SweepResult :type "HitResult Structure (by ref)"))
  (`self.HitActor` OtherActor))

(event `self.RamCollider.OnComponentHit`
  (params (HitComponent :type "PrimitiveComponent Object Reference") (OtherActor :type "Actor Object Reference") (OtherComp :type "PrimitiveComponent Object Reference") (NormalImpulse :type "Vector Structure") (Hit :type "HitResult Structure (by ref)"))
  (`self.HitActor` OtherActor))

(fn `HitActor`
  (params (HitActor :type "Actor Object Reference"))
  (if (and (`self.bRamming`) (!= HitActor (`self.GetParentActor`)))
    (cast `StaticMeshActor` (`local.HitActor`)
      (:`then`
        (`self.HitStaticObject`)
        (return))
      (:`CastFailed`
        (bind _aspawn (cast `Pawn` (`local.HitActor`)))
        (`/Engine/EditorBlueprintResources/StandardMacros.IsValid` _aspawn
          (:`Is Valid`
            (message `/Game/Unicorn/Core/Engine/BPI_Knockback.Knockback` _aspawn (`self.K2_GetActorLocation`) (`self.KnockbackForce`))
            (message `/Game/Unicorn/Core/Engine/BPI_Stunnable.BeStunned` (`local.HitActor`) (`self.StunPower`))
            (message `HealthInterface.LoseHealth` (`local.HitActor`) (`self.RamDamage`))
            (`self.HitDamageableObject`)
            (return)))))))

(fn `HitEnemy`
  (params (NewParam :type "Actor Object Reference")))

(fn `SetRamming`
  (params (NewRamming :type Boolean))
  (bind _output_get (set `self.bRamming` NewRamming))
  (if _output_get
    (`MaterialInstanceDynamic.SetVectorParameterValue` (`self.ShieldMat`) (`UnicornMaterialParameters.Color`) (`self.RamColor`))
    (`MaterialInstanceDynamic.SetScalarParameterValue` (`self.ShieldMat`) (`UnicornMaterialParameters.Emissive`) (`self.RammingEmissive`))
    (else
      (`MaterialInstanceDynamic.SetVectorParameterValue` (`self.ShieldMat`) (`UnicornMaterialParameters.Color`) (`self.NormalColor`))))
  (return))

(fn `UserConstructionScript`
  (`parent.UserConstructionScript`)
  (bind _returnvalue (`KismetMaterialLibrary.CreateDynamicMaterialInstance` "/Game/Unicorn/Spells/M_StaticShield.M_StaticShield"))
  (bind _output_get (set `self.ShieldMat` _returnvalue))
  (`PrimitiveComponent.SetMaterial` (`self.Mesh`) 0 _output_get)
  (`MaterialInstanceDynamic.SetVectorParameterValue` (`self.ShieldMat`) (`UnicornMaterialParameters.Color`) (`self.NormalColor`)))