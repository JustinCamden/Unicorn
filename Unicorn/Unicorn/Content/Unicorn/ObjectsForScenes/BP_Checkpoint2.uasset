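; BP_Checkpoint2 is a scene checkpoint actor that shows a text label and removes itself once its clear condition is met.
; On BeginPlay it copies its Text into the Widget_BillboardText of its CheckPointText component.
; It destroys itself when Tick finds the EnemyLeft reference invalid, or when DecreaseIceBlock counts IceBlocksLeft down to zero, printing the remaining count until then.
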(event `self.ReceiveBeginPlay`
  (bind _aswidget_billboard_text (cast `/Game/Unicorn/ObjectsForScenes/Widget_BillboardText` (`WidgetComponent.GetUserWidgetObject` (`self.CheckPointText`))))
  (set `/Game/Unicorn/ObjectsForScenes/Widget_BillboardText.Text` (`self.text`) _aswidget_billboard_text))

(event `self.ReceiveActorBeginOverlap`
  (params (OtherActor :type "Actor Object Reference")))

(event `self.ReceiveTick`
  (params (DeltaSeconds :type "Float (single-precision)"))
  (`/Engine/EditorBlueprintResources/StandardMacros.IsValid` (`self.enemyLeft`)
    (:`Is Not Valid`
      (`self.K2_DestroyActor`))))

(fn `DecreaseIceBlock`
  (bind _ice_blocks_left (`self.Ice_Blocks_Left`))
  (`/Engine/EditorBlueprintResources/StandardMacros.DecrementInt` _ice_blocks_left
    (:`  `
      (if (== _ice_blocks_left 0)
        (`self.K2_DestroyActor`)
        (else
          (`KismetSystemLibrary.PrintString` (`KismetStringLibrary.Conv_IntToString` _ice_blocks_left)))))))

(fn `UserConstructionScript`)