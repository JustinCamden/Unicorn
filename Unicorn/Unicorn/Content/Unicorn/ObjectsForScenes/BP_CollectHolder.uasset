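; BP_CollectHolder is a drop-off point where the player deposits carried collectibles.
; On overlap with BP_PlayerCharacter, it decrements a non-zero NumOfCollectibles, spawns BP_Collectible_Collected, sets GemDropped and prints debug text.
; The spawn uses the holder's rotation and X/Z location, but Y reads from an increment node that never executes.
; GemDropped is never checked, so repeat overlaps can deposit again.
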(event EventBeginPlay)

(event Collision|EventActorBeginOverlap
  (params (OtherActor :type Actor%20Object%20Reference))
  (bind _returnvalue (Transformation|GetActorLocation))
  (bind _asbp_player_character (Utilities|Casting|CastToBP_PlayerCharacter OtherActor))
  (if (> (Variables|/Game/Unicorn/Characters/Player/BP_PlayerCharacter.BP_PlayerCharacter_C|GetNumOfCollectibles _asbp_player_character) 0)
    (bind _result (Math|Integer|DecrementInt (Variables|/Game/Unicorn/Characters/Player/BP_PlayerCharacter.BP_PlayerCharacter_C|GetNumOfCollectibles _asbp_player_character))
      (:%20%20
        (Game|SpawnActorfromClass "/Game/Unicorn/ObjectsForScenes/BP_Collectible_Collected.BP_Collectible_Collected_C" (Math|Transform|MakeTransform (Math|Vector|MakeVector (.x _returnvalue) (stale _result) (.z _returnvalue)) (Transformation|GetActorRotation)) "Undefined" 0 0)
        (Variables|Default|SetGemDropped true)
        (Development|PrintString "Gem dropped")
        (Development|PrintString (Utilities|String|ToString(Integer) _result))))))

(event EventTick
  (params (DeltaSeconds :type Float%20%28single-precision%29)))

(fn ConstructionScript)