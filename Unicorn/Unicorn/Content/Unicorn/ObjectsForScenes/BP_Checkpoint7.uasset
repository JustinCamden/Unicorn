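; BP_Checkpoint7 is a scene object, apparently an ice-block barrier, that disappears once its gem count runs out.
; DecreaseIceBlock decrements GemsLeft, destroying the actor at zero and otherwise printing the remaining count.
; The file shows no caller for that function; the overlap event is empty, Tick is disabled, and an unconnected copy of the countdown logic remains in the EventGraph.
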(event `self.ReceiveActorBeginOverlap`
  (params (OtherActor :type "Actor Object Reference")))

(fn `DecreaseIceBlock`
  (bind _gems_left (`self.Gems_Left`))
  (`/Engine/EditorBlueprintResources/StandardMacros.DecrementInt` _gems_left
    (:`  `
      (if (== _gems_left 0)
        (`self.K2_DestroyActor`)
        (else
          (`KismetSystemLibrary.PrintString` (`KismetStringLibrary.Conv_IntToString` _gems_left)))))))

(fn `UserConstructionScript`)