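; BP_Checkpoint is a scene actor that displays a text billboard and removes itself once its ice block count runs out.
; On BeginPlay it copies its Text variable into the Billboard_Text widget of the CheckPointText component.
; DecreaseIceBlock decrements IceBlocksLeft, destroys the actor at zero and otherwise prints the remaining count.
; Nothing in this Blueprint calls that function, and the overlap event is empty.
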(event `self.ReceiveBeginPlay`
  (bind _asbillboard_text (cast `/Game/Unicorn/ObjectsForScenes/Billboard_Text` (`WidgetComponent.GetUserWidgetObject` (`self.CheckPointText`))))
  (set `/Game/Unicorn/ObjectsForScenes/Billboard_Text.Text` (`self.text`) _asbillboard_text))

(event `self.ReceiveActorBeginOverlap`
  (params (OtherActor :type "Actor Object Reference")))

(fn `DecreaseIceBlock`
  (bind _ice_blocks_left (`self.Ice_Blocks_Left`))
  (`/Engine/EditorBlueprintResources/StandardMacros.DecrementInt` _ice_blocks_left
    (:`  `
      (if (== _ice_blocks_left 0)
        (`self.K2_DestroyActor`)
        (else
          (`KismetSystemLibrary.PrintString` (`KismetStringLibrary.Conv_IntToString` _ice_blocks_left)))))))

(fn `UserConstructionScript`)