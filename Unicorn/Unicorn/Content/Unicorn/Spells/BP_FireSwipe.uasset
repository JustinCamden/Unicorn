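; BP_FireSwipe is a spell actor that sweeps by rotating toward an offset from its spawn orientation.
; On BeginPlay it derives a target rotation from RotationDelta in local space, then a timer delays the start of turning.
; Once turning, Tick eases the actor toward that target with RInterpTo at TurningSpeed.
; DeactivateSpell only defers to the parent class.
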(event `self.ReceiveBeginPlay`
  (`parent.ReceiveBeginPlay`)
  (set `self.StartRotation` (`self.K2_GetActorRotation`))
  (set `self.TargetRotation` (`KismetMathLibrary.TransformRotation` (`self.GetTransform`) (`self.RotationDelta`)))
  (`KismetSystemLibrary.K2_SetTimerDelegate` (delegate `BeginTurning`) (`self.TurningDelayTimer`)))

(event `BeginTurning`
  (set `self.bTurning` true))

(event `self.ReceiveTick`
  (params (DeltaSeconds :type "Float (single-precision)"))
  (`parent.ReceiveTick` DeltaSeconds)
  (if (`self.bTurning`)
    (`self.K2_SetActorRotation` (`KismetMathLibrary.RInterpTo` (`self.K2_GetActorRotation`) (`self.TargetRotation`) (`GameplayStatics.GetWorldDeltaSeconds`) (`self.TurningSpeed`)))))

(event `/Game/Unicorn/Spells/BP_Spell_Base.DeactivateSpell`
  (`parent.DeactivateSpell`))

(fn `UserConstructionScript`
  (`parent.UserConstructionScript`))