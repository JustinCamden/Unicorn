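; BP_IceSpike is an ice spike spell actor that inherits its begin play, overlap and tick behavior from a parent class.
; Its construction script sets the life span to zero, so it has no timed expiry from that setting.
; Its Deflect override runs the parent's deflect logic, then turns the actor to face opposite its current forward vector and reports success.
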(event `self.ReceiveBeginPlay`
  (`parent.ReceiveBeginPlay`))

(event `self.ReceiveActorBeginOverlap`
  (params (OtherActor :type "Actor Object Reference"))
  (`parent.ReceiveActorBeginOverlap` OtherActor))

(event `self.ReceiveTick`
  (params (DeltaSeconds :type "Float (single-precision)"))
  (`parent.ReceiveTick` DeltaSeconds))

(fn `Deflect`
  (params (DeflectorDirection :type "Vector Structure") (DeflectorTeam :type "ETeam Enum" :default "TE_Player") (DeflectorEnemyTeam :type "ETeam Enum" :default "TE_Player"))
  (returns (Success :type Boolean))
  (`parent.Deflect` DeflectorDirection DeflectorTeam DeflectorEnemyTeam)
  (`self.K2_SetActorRotation` (`KismetMathLibrary.MakeRotFromX` (* (`self.GetActorForwardVector`) -1.0)))
  (return true))

(fn `UserConstructionScript`
  (`parent.UserConstructionScript`)
  (`self.SetLifeSpan` 0.0))