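; BP_FireSideSwipe is a fire spell projectile that starts turning toward a target rotation after a delay.
; A one-shot timer on BeginPlay handles the delay, with a Turning flag gating the steering in Tick.
; While turning, it interpolates actor rotation with RInterpTo and reapplies ProjectileVelocity in local space, so its travel path curves with its facing.
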(event `self.ReceiveBeginPlay`
  (`parent.ReceiveBeginPlay`)
  (`KismetSystemLibrary.K2_SetTimerDelegate` (`|CreateDelegate` :!event `BeginTurning`) (`self.TurningDelayTime`)))

(event `BeginTurning`
  (set `self.bTurning` true))

(event `self.ReceiveTick`
  (params (DeltaSeconds :type "Float (single-precision)"))
  (`parent.ReceiveTick` DeltaSeconds)
  (if (`self.bTurning`)
    (`self.K2_SetActorRotation` (`KismetMathLibrary.RInterpTo` (`self.K2_GetActorRotation`) (`self.TargetRotation`) (`GameplayStatics.GetWorldDeltaSeconds`) (`self.TurningSpeed`)))
    (`ProjectileMovementComponent.SetVelocityInLocalSpace` (`self.ProjectileMovement`) (`self.ProjectileVelocity`))))

(event `/Game/Unicorn/Spells/BP_Spell_Base.DeactivateSpell`
  (`parent.DeactivateSpell`))

(fn `UserConstructionScript`
  (`parent.UserConstructionScript`))