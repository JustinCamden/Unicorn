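; BP_BodyShield is a spell that shows a collidable forcefield mesh while active and signals a deflection when an ice spike overlaps it.
; Its Health resource drives a dynamic material parameter, and losing it all breaks and deactivates the shield.
; While inactive, Tick plays a timeline that scales regeneration and restarts on damage.
; A broken shield cannot reactivate until that regeneration reaches full health.
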(event `self.ReceiveBeginPlay`
  (`HealthInterface.GainHealth` 0.0))

(event `self.ReceiveTick`
  (params (DeltaSeconds :type "Float (single-precision)"))
  (`parent.ReceiveTick` DeltaSeconds)
  ;[1 1 1] Handle regaining health when inactive
  (if (`self.bSpellActive`)
    _
    (elif (not (`ResourceComponent.IsAtMaxCapacity` (`self.Health`)))
      (bind (_direction _healthregenpercent) (`Timeline|HealthRegenTimeline`)
        (:`Update`
          (`HealthInterface.GainHealth` (* _healthregenpercent (`self.BaseHealthRegenPerSecond`)))
          (if (`ResourceComponent.IsAtMaxCapacity` (`self.Health`))
            (set `self.bBroken` false)))))))

(event `self.DeactivateSpell`
  (`parent.DeactivateSpell`)
  (`SceneComponent.SetVisibility` (`self.ShieldMesh`) false false)
  (`PrimitiveComponent.SetCollisionEnabled` (`self.ShieldMesh`) "NoCollision"))

(event `self.ActivateSpell`
  ;[1 1 1] Only activate if the spell isn't broken
  (if (not (`self.bBroken`))
    (`parent.ActivateSpell`)
    (`SceneComponent.SetVisibility` (`self.ShieldMesh`) true false)
    (`PrimitiveComponent.SetCollisionEnabled` (`self.ShieldMesh`) "QueryOnly")))

(event `OnShieldBreak`
  ;[1 1 1] Update broken status and deactivate the spell when we lose all our health
  (set `self.bBroken` true)
  (`self.DeactivateSpell`))

(event `self.ReceiveActorBeginOverlap`
  (params (OtherActor :type "Actor Object Reference"))
  (cast `/Game/Unicorn/Spells/BP_IceSpike` OtherActor)
  (`self.OnShieldDeflected`))

(fn `GainHealth`
  (params (HealthGained :type "Float (double-precision)"))
  (returns (ReturnValue :type Boolean))
  (bind _health (`self.Health`))
  (`ResourceComponent.GainResource` (`self.Health`) HealthGained)
  (`MaterialInstanceDynamic.SetScalarParameterValue` (`self.ShieldMatRef`) "Health" (/ (`ResourceComponent.CurrentResource` _health) (`ResourceComponent.MaxResource` _health)))
  (return true))

(fn `GetCurrHealthPercent`
  (returns (ReturnValue :type "Float (double-precision)"))
  (bind _health (`self.Health`))
  (return (/ (`ResourceComponent.CurrentResource` _health) (`ResourceComponent.MaxResource` _health))))

(fn `LoseHealth`
  (params (HealthLost :type "Float (double-precision)"))
  (returns (bDied :type Boolean) (ReturnValue :type Boolean))
  (locals (LocalDied :type Boolean :default false))
  (bind _bdepleted (`ResourceComponent.LoseResource` (`self.Health`) HealthLost))
  (set `local.LocalDied` _bdepleted)
  (`MaterialInstanceDynamic.SetScalarParameterValue` (`self.ShieldMatRef`) "Health" (`self.GetCurrHealthPercent`))
  (`|ExecutionSequence`
    (:`then_0`
      (if (`local.LocalDied`)
        (`self.OnShieldBreak`)))
    (:`then_1`
      (`TimelineComponent.SetNewTime` (`self.HealthRegenTimeline`) 0.0)
      (return (`local.LocalDied`) true))))

(fn `UserConstructionScript`
  ;[1 1 1] Get a reference to our forcefield mat so we can adjust it later
  (bind _returnvalue (`KismetMaterialLibrary.CreateDynamicMaterialInstance` (`self.ShieldMat`)))
  (bind _output_get (set `self.ShieldMatRef` _returnvalue))
  (`PrimitiveComponent.SetMaterial` (`self.ShieldMesh`) 0 _output_get))