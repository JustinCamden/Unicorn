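; BP_DeflectionShield is a shield spell that deflects enemy actors overlapping it while it is moved fast enough.
; While active, Tick compares kinematic velocity to a minimum, playing or reversing a timeline whose completion toggles deflection and swaps the shield and deflection meshes, so switching is delayed.
; Overlapping enemies receive a deflect message with the shield's forward vector and player team data.
; Deactivating the spell resets deflection and the timeline.
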(event `self.ReceiveActorBeginOverlap`
  (params (OtherActor :type "Actor Object Reference"))
  (`parent.ReceiveActorBeginOverlap` OtherActor)
  (if (`self.bDeflecting`)
    (if (`TeamComponent.IsEnemyTeam` (`self.Team`) OtherActor)
      (message `/Game/Unicorn/Spells/BPI_Deflectable.Deflect` OtherActor (`self.GetActorForwardVector`) "TE_Player" "TE_PlayerEnemy"))))

(event `self.ReceiveTick`
  (params (DeltaSeconds :type "Float (single-precision)"))
  (`parent.ReceiveTick` DeltaSeconds)
  (if (`self.bSpellActive`)
    ;[1 1 1] If active, check if we are at or above the min activation velocity
    (if (<= (`self.MinDeflectionVelocity`) (`KismetMathLibrary.VSize` (`/Game/Unicorn/Core/Engine/BP_KinematicVelocity_Component.GetKinematicVelocity` (`self.KinematicVelocityRef`))))
      ;[1 1 1] Progress or reduce the timeline accordingly
      (bind _direction (`Timeline|ActivationToggleTimeline` :!label _label)
        (:`Finished`
          (switch `ETimelineDirection` _direction
            (:`Forward`
              ;[1 1 1] When finished, activate or deactivate the deflection as necessary
              (if (not (`self.bDeflecting`))
                (set `self.bDeflecting` true)
                (`SceneComponent.SetVisibility` (`self.ShieldMesh`) false false)
                (`SceneComponent.SetVisibility` (`self.DeflectionMesh`) true false)))
            (:`Backward`
              (if (`self.bDeflecting`)
                (set `self.bDeflecting` false)
                (`SceneComponent.SetVisibility` (`self.ShieldMesh`) true false)
                (`SceneComponent.SetVisibility` (`self.DeflectionMesh`) false false))))))
      (else
        (goto _label :!via `Reverse`)))))

(event `self.DeactivateSpell`
  (`parent.DeactivateSpell`)
  (`SceneComponent.SetVisibility` (`self.DeflectionMesh`) false false)
  (set `self.bDeflecting` false)
  (`TimelineComponent.SetNewTime` (`self.ActivationToggleTimeline`) 0.0))

(fn `IsDeflecting`
  (returns (ReturnValue :type Boolean))
  (return (`self.bDeflecting`)))

(fn `UserConstructionScript`
  (`parent.UserConstructionScript`)
  (bind _returnvalue (`KismetMaterialLibrary.CreateDynamicMaterialInstance` (`self.DeflectionMat`)))
  (bind _output_get (set `self.DeflectionMatRef` _returnvalue))
  (`PrimitiveComponent.SetMaterial` (`self.DeflectionMesh`) 0 _output_get))