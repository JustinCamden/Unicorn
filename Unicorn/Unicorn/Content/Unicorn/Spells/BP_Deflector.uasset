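; BP_Deflector is a spell that forms a forcefield shield which deflects overlapping objects not on the caster's team.
; It deflects only while the spell is active and the kinematic tracker reports movement above a minimum velocity.
; Tick toggles mesh visibility and query collision to match that state.
; On overlap it sends a deflect message carrying the shield's forward vector and team info.
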(event `self.ReceiveActorBeginOverlap`
  (params (OtherActor :type "Actor Object Reference"))
  ;[1 1 1] If deflecting, deflect actors in the direction the shield is facing
  (bind _returnvalue (`self.IsDeflecting`))
  (if _returnvalue
    (if (not (`TeamComponent.IsSameTeam` (`self.Team`) OtherActor))
      (message `/Game/Unicorn/Spells/BPI_Deflectable.Deflect` OtherActor (`self.GetActorForwardVector`) (`TeamComponent.Team` (`self.Team`)) (`TeamComponent.EnemyTeam` (`self.Team`))))))

(event `self.ReceiveTick`
  (params (DeltaSeconds :type "Float (single-precision)"))
  ;[1 1 1] Handle enabling and disabling the collision and visibility
  (bind _returnvalue (`self.IsDeflecting`))
  (if _returnvalue
    (if (not (`SceneComponent.IsVisible` (`self.Mesh`)))
      (`SceneComponent.SetVisibility` (`self.Mesh`) true false)
      (`PrimitiveComponent.SetCollisionEnabled` (`self.Mesh`) "QueryOnly"))
    (elif (`SceneComponent.IsVisible` (`self.Mesh`))
      (`SceneComponent.SetVisibility` (`self.Mesh`) false false)
      (`PrimitiveComponent.SetCollisionEnabled` (`self.Mesh`) "NoCollision"))))

(event `self.ActivateSpell`
  (`parent.ActivateSpell`))

(event `self.DeactivateSpell`
  (`parent.DeactivateSpell`))

(fn `IsDeflecting`
  (returns (ReturnValue :type Boolean))
  (if (`self.bSpellActive`)
    ;[1 1 1] Check whether we are moving fast enough to deflect projectiles
    (return (>= (`KismetMathLibrary.VSize` (`/Game/Unicorn/Core/Engine/BP_KinematicVelocity_Component.GetKinematicVelocity` (`self.KinematicTracker`))) (`self.MinActivationVelocity`)))
    (else
      (return false))))

(fn `UserConstructionScript`
  ;[1 1 1] Get a reference to our forcefield mat so we can adjust it later
  (bind _returnvalue (`KismetMaterialLibrary.CreateDynamicMaterialInstance` "/Game/Unicorn/Spells/M_ForceField.M_ForceField"))
  (bind _output_get (set `self.ForceFieldMat` _returnvalue))
  (`PrimitiveComponent.SetMaterial` (`self.Mesh`) 0 _output_get))