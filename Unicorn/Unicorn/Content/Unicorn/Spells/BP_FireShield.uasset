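; BP_FireShield is a spell actor for a fire shield with health, a limited lifetime and a VR owner.
; A timeline scales the mesh up on spawn, then plays in reverse on deactivation before destroying the actor.
; Lifetime expiry, depleted health or the owner moving horizontally beyond the shield's radius deactivates it.
; Health changes feed a dynamic forcefield material's Health parameter.
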(event `self.ReceiveBeginPlay`
  (`self.ActivateSpell`)
  (set `self.CurrShieldGrowthState` "NewEnumerator1")
  (`GameplayStatics.SpawnSoundAttached` "/Game/ProSoundCollection_v1_3/Magic_Spells/Cues/casting_charge_whoosh_buildup4_Cue.casting_charge_whoosh_buildup4_Cue" (`self.RootComponent`) "None" (0.0 0.0 0.0) (struct) "KeepRelativeOffset" false 1.0 1.0 0.0 "/Game/ATT_Spell.ATT_Spell" "/Game/CON_Spell.CON_Spell"))

(event `self.ReceiveTick`
  (params (DeltaSeconds :type "Float (single-precision)"))
  (bind (_relativescale3d_x _relativescale3d_y _relativescale3d_z) (`KismetMathLibrary.BreakVector` (`SceneComponent.RelativeScale3D` (`self.ShieldMesh`))))
  (`parent.ReceiveTick` DeltaSeconds)
  (`|ExecutionSequence`
    (:`then_0`
      ;[1 1 1] Handle growing and shrinking the shield when spawning and dying
      (switch `/Game/Unicorn/Core/Engine/EGrowthState` (`self.CurrShieldGrowthState`)
        (:`NewEnumerator1`
          (bind (_direction _growth) (`Timeline|GrowthTimeline` :!label _label)
            (:`Update`
              (`SceneComponent.SetRelativeScale3D` (`self.ShieldMesh`) (`KismetMathLibrary.VLerp` (`self.ShieldMinSize`) (`self.ShieldMaxSize`) _growth)))
            (:`Finished`
              (switch `ETimelineDirection` _direction
                (:`Forward`
                  (set `self.CurrShieldGrowthState` "NewEnumerator3")
                  ;[1 1 1] Set a deactivation timer as appropriate
                  (bind _returnvalue (`KismetSystemLibrary.K2_SetTimerDelegate` (delegate `OnLifetimeTimerExpired`) (`self.ShieldLifetime`)))
                  (set `self.ShieldLifetimeTmer` _returnvalue))
                (:`Backward`
                  (`self.K2_DestroyActor`))))))
        (:`NewEnumerator2`
          (goto _label :!via `Reverse`))))
    (:`then_1`
      ;[1 1 1] Deactivate the spell when we get too far away
      (if (`self.bSpellActive`)
        (if (> (`KismetMathLibrary.VSize` (`/Game/Unicorn/Core/Engine/BPFL_UnicornLibrary.FlattenZ` (- (`VRBaseCharacter.GetVRLocation` (`self.ShieldOwner`)) (`self.K2_GetActorLocation`)))) (* (`.SphereRadius` (`KismetSystemLibrary.GetComponentBounds` (`self.ShieldMesh`))) (/ _relativescale3d_x _relativescale3d_z)))
          (`KismetSystemLibrary.K2_ClearAndInvalidateTimerHandle` (`self.ShieldLifetimeTmer`))
          (`self.DeactivateSpell`))))))

(event `OnLifetimeTimerExpired`
  ;[1 1 1] Set a deactivation timer as appropriate
  (`self.DeactivateSpell`))

(event `self.DeactivateSpell`
  (`parent.DeactivateSpell`)
  (set `self.CurrShieldGrowthState` "NewEnumerator2"))

(fn `GainHealth`
  (params (HealthGained :type "Float (double-precision)"))
  (returns (ReturnValue :type Boolean))
  (bind _health (`self.Health`))
  (`ResourceComponent.GainResource` (`self.Health`) HealthGained)
  (`MaterialInstanceDynamic.SetScalarParameterValue` (`self.ShieldMatRef`) "Health" (/ (`ResourceComponent.CurrentResource` _health) (`ResourceComponent.MaxResource` _health)))
  (return true))

(fn `GetCurrHealthPercent`
  (returns (ReturnValue :type "Float (double-precision)"))
  (bind _health (`self.Health`))
  (return (/ (`ResourceComponent.CurrentResource` _health) (`ResourceComponent.MaxResource` _health))))

(fn `LoseHealth`
  (params (HealthLost :type "Float (double-precision)"))
  (returns (bDied :type Boolean) (ReturnValue :type Boolean))
  (locals (bLocalDied :type Boolean :default false))
  (bind _bdepleted (`ResourceComponent.LoseResource` (`self.Health`) HealthLost))
  (set `local.bLocalDied` _bdepleted)
  (`MaterialInstanceDynamic.SetScalarParameterValue` (`self.ShieldMatRef`) "Health" (`self.GetCurrHealthPercent`))
  (`|ExecutionSequence`
    (:`then_0`
      (if (`local.bLocalDied`)
        (`KismetSystemLibrary.K2_ClearAndInvalidateTimerHandle` (`self.ShieldLifetimeTmer`))
        (`self.DeactivateSpell`))
      (return (`local.bLocalDied`) true))))

(fn `UserConstructionScript`
  ;[1 1 1] Get a reference to our forcefield mat so we can adjust it later
  (bind _returnvalue (`KismetMaterialLibrary.CreateDynamicMaterialInstance` (`self.ShieldMat`)))
  (bind _output_get (set `self.ShieldMatRef` _returnvalue))
  (`PrimitiveComponent.SetMaterial` (`self.ShieldMesh`) 0 _output_get))