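; BP_Fireball is a projectile spell that damages the first valid non-friendly actor it hits, then destroys itself.
; Overlaps, including those present at spawn, go through HitActor, which checks spell activity, team and target deflection before sending a damage message.
; Tick reapplies local-space velocity to keep speed constant, and the construction script sets its lifespan.
; Deflect hands the fireball to the deflector's team and reverses its velocity.
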(event `self.ReceiveBeginPlay`
  (`parent.ReceiveBeginPlay`)
  (`self.ActivateSpell`)
  (for _array_element (`self.GetOverlappingActors` null)
    (`self.HitActor` _array_element)))

(event `self.ReceiveActorBeginOverlap`
  (params (OtherActor :type "Actor Object Reference"))
  (`self.HitActor` OtherActor))

(event `self.ReceiveTick`
  (params (DeltaSeconds :type "Float (single-precision)"))
  (`parent.ReceiveTick` DeltaSeconds)
  ;[1 1 1] Ensure that we move at the same rate every tick
  (`ProjectileMovementComponent.SetVelocityInLocalSpace` (`self.ProjectileMovement`) (`self.ProjectileVelocity`)))

(fn `Deflect`
  (params (DeflectorDirection :type "Vector Structure") (DeflectorTeam :type "ETeam Enum" :default "TE_Player"))
  (returns (Success :type Boolean))
  (bind _output_get (set `self.SpellTeam` DeflectorTeam))
  (set `TeamComponent.Team` _output_get (`self.Team`))
  (set `self.ProjectileVelocity` (* (`self.ProjectileVelocity`) -1.0))
  (return true))

(fn `HitActor`
  (params (InputPin :type "Actor Object Reference"))
  ;[1 1 1] Check if we are active
  (if (`self.bSpellActive`)
    ;[1 1 1] Check in the overlapped actor is the same team (we don't want friendly fire)
    (if (not (`TeamComponent.IsSameTeam` (`self.Team`) InputPin))
      ;[1 1 1] Check if the other actor is currently deflecting
      (bind _returnvalue (message `/Game/Unicorn/Spells/BPI_Deflector.IsDeflecting` InputPin))
      (if (not _returnvalue)
        ;[1 1 1] If all the conditions are cleared, damage the other actor and destroy this fireball
        (message `HealthInterface.LoseHealth` InputPin (`self.DamageAmount`))
        (`self.K2_DestroyActor`)))))

(fn `UserConstructionScript`
  (`parent.UserConstructionScript`)
  (`self.SetLifeSpan` (`self.Lifetime`)))