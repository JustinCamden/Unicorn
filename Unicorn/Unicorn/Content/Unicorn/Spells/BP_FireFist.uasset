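; BP_FireFist is a melee punch spell that hurts enemies struck by a fast-moving fist.
; Tick compares KinematicTracker speed to a minimum to flag punch velocity.
; While the spell is active, overlapping an actor on another team at that speed sends knockback, stun and damage messages.
; Such hits also start a blast sphere state machine, which scales the sphere up and back down through a forward-then-reversed timeline.
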(event `self.ReceiveBeginPlay`
  (`parent.ReceiveBeginPlay`))

(event `self.ReceiveActorBeginOverlap`
  (params (OtherActor :type "Actor Object Reference"))
  (`parent.ReceiveActorBeginOverlap` OtherActor)
  (if (`self.bSpellActive`)
    (`self.HitActor` OtherActor)))

(event `self.ReceiveTick`
  (params (DeltaSeconds :type "Float (single-precision)"))
  (bind _blastsphere (`self.BlastSphere`))
  (`parent.ReceiveTick` DeltaSeconds)
  (`|ExecutionSequence`
    (:`then_0`
      ;[1 1 1] Update whether we are at punch velocity
      (set `self.bAtPunchVelocity` (>= (`KismetMathLibrary.VSize` (`/Game/Unicorn/Core/Engine/BP_KinematicVelocity_Component.GetKinematicVelocity` (`self.KinematicTracker`))) (`self.MinPunchVelocity`))))
    (:`then_1`
      ;[1 1 1] Handle growing and shrinking the blast sphere after we hit an actor
      (switch `/Game/Unicorn/Core/Engine/EGrowthState` (`self.BlastSphereState`)
        (:`NewEnumerator1`
          (bind (_direction _blastspheresize) (`Timeline|BlastSphereSTimeline` :!label _label)
            (:`Update`
              (`SceneComponent.SetRelativeScale3D` (`self.BlastSphere`) (`KismetMathLibrary.VLerp` (0.0 0.0 0.0) (`self.BlastSphereMaxSize`) _blastspheresize)))
            (:`Finished`
              (switch `ETimelineDirection` _direction
                (:`Forward`
                  (set `self.BlastSphereState` "NewEnumerator2"))
                (:`Backward`
                  (set `self.BlastSphereState` "NewEnumerator0"))))
            (:`ToggleBlastSphereVisibility`
              (`SceneComponent.SetVisibility` _blastsphere (not (`SceneComponent.bVisible` _blastsphere)) false))))
        (:`NewEnumerator2`
          (goto _label :!via `Reverse`))))))

(fn `HitActor`
  (params (HitActor :type "Actor Object Reference"))
  ;[1 1 1] If we hit an enemy actor and are at punch velocity, damage that enemy and knock them back
  (if (`TeamComponent.IsSameTeam` (`self.Team`) HitActor)
    _
    (elif (`self.bAtPunchVelocity`)
      (message `/Game/Unicorn/Core/Engine/BPI_Knockback.Knockback` (`local.HitActor`) (`SceneComponent.K2_GetComponentLocation` (`self.Sphere`)) (`self.KnockbackForce`))
      (message `/Game/Unicorn/Core/Engine/BPI_Stunnable.BeStunned` (`local.HitActor`) (`self.StunPower`))
      (message `HealthInterface.LoseHealth` (`local.HitActor`) (`self.DamageAmount`))
      (set `self.BlastSphereState` "NewEnumerator1")
      (return))))

(fn `UserConstructionScript`
  (`parent.UserConstructionScript`))