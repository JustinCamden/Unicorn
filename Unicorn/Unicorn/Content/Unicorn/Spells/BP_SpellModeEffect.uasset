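; BP_SpellModeEffect is a spell effect that shows the current casting mode as a hand effect with a Fire or Force material.
; Activating the spell reveals HandEffect and sets a growth state, which Tick uses to play or reverse a timeline that scales it between MinSize and MaxSize.
; Deactivation shrinks the effect, then hides it when the timeline finishes backward.
; SwitchCastingMode swaps the material, or safely deactivates the spell when not casting.
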(event `self.ReceiveTick`
  (params (DeltaSeconds :type "Float (single-precision)"))
  (`parent.ReceiveTick` DeltaSeconds)
  (switch `/Game/Unicorn/Core/Engine/EGrowthState` (`self.CurrGrowthState`)
    (:`NewEnumerator1`
      (bind (_direction _handeffectsize) (`Timeline|GrowthTimeline` :!label _label)
        (:`Update`
          (`SceneComponent.SetRelativeScale3D` (`self.HandEffect`) (`KismetMathLibrary.VLerp` (`self.MinSize`) (`self.MaxSize`) _handeffectsize)))
        (:`Finished`
          (switch `ETimelineDirection` _direction
            (:`Forward`
              (set `self.CurrGrowthState` "NewEnumerator3"))
            (:`Backward`
              (set `self.CurrGrowthState` "NewEnumerator0")
              (`SceneComponent.SetVisibility` (`self.HandEffect`) false false))))))
    (:`NewEnumerator2`
      (goto _label :!via `Reverse`))))

(event `self.ActivateSpell`
  (`parent.ActivateSpell`)
  (`SceneComponent.SetVisibility` (`self.HandEffect`) true false)
  (set `self.CurrGrowthState` "NewEnumerator1"))

(event `self.DeactivateSpell`
  (set `self.CurrGrowthState` "NewEnumerator2"))

(fn `SwitchCastingMode`
  (params (CastingMode :type "/Game/Unicorn/Core/Engine/ESpellcastingMode Enum" :default "NewEnumerator0"))
  (switch `/Game/Unicorn/Core/Engine/ESpellcastingMode` CastingMode
    (:`NewEnumerator0`
      (`self.SafeDeactivateSpell`))
    (:`NewEnumerator2`
      (`PrimitiveComponent.SetMaterial` (`self.HandEffect`) 0 (`self.FireMasterial`)))
    (:`NewEnumerator3`
      (`PrimitiveComponent.SetMaterial` (`self.HandEffect`) 0 (`self.ForceMaterial`))))
  (return))

(fn `UserConstructionScript`
  (`parent.UserConstructionScript`))