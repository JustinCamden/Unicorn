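; Shield spell that toggles a force-field mesh and its collision on activation, with its own health pool.
; LoseHealth restarts the regen timeline and breaks the shield on depletion, blocking activation until health refills.
; While inactive, Tick plays that timeline to scale regeneration.
; Health changes recolor a dynamic material through healthy, damaged and dead colors, though the ratio is computed as max over current health.
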(event `self.ReceiveBeginPlay`
  (`self.GainHealth` 0.0))

(event `self.ReceiveTick`
  (params (DeltaSeconds :type "Float (single-precision)"))
  (`parent.ReceiveTick` DeltaSeconds)
  ;[1 1 1] Handle regaining health when inactive
  (if (`self.bSpellActive`)
    _
    (elif (not (`ResourceComponent.IsAtMaxCapacity` (`self.Health`)))
      (bind (_direction _healthregenpercent) (`Timeline|HealthRegenTimeline`)
        (:`Update`
          (`self.GainHealth` (* _healthregenpercent (`self.BaseHealthRegenPerSecond`)))
          (if (`ResourceComponent.IsAtMaxCapacity` (`self.Health`))
            (set `self.bBroken` false)))))))

(event `self.ActivateSpell`
  (if (not (`self.bBroken`))
    (`parent.ActivateSpell`)
    (`SceneComponent.SetVisibility` (`self.Mesh`) true false)
    (`PrimitiveComponent.SetCollisionEnabled` (`self.Mesh`) "QueryOnly")
    (`PrimitiveComponent.SetCollisionEnabled` (`self.Box`) "QueryOnly")))

(event `OnShieldBreak`
  (set `self.bBroken` true)
  (`self.DeactivateSpell`))

(event `self.DeactivateSpell`
  (`parent.DeactivateSpell`)
  (`SceneComponent.SetVisibility` (`self.Mesh`) false false)
  (`PrimitiveComponent.SetCollisionEnabled` (`self.Mesh`) "NoCollision")
  (`PrimitiveComponent.SetCollisionEnabled` (`self.Box`) "NoCollision"))

(fn `GainHealth`
  (params (HealthGained :type "Float (double-precision)"))
  (returns (ReturnValue :type Boolean))
  (`ResourceComponent.GainResource` (`self.Health`) HealthGained)
  (`MaterialInstanceDynamic.SetVectorParameterValue` (`self.ForceFieldMat`) (`UnicornMaterialParameters.Color`) (`self.GetForceFieldColor`))
  (return true))

(fn `GetForceFieldColor`
  (returns (ReturnValue :type "LinearColor Structure"))
  (locals (HealthLevel :type "Float (double-precision)" :default 0.0))
  (bind _health (`self.Health`))
  ;[1 1 1] Get the current health percent
  (bind _output_get (set `local.HealthLevel` (/ (`ResourceComponent.MaxResource` _health) (`ResourceComponent.CurrentResource` _health))))
  (if (> _output_get 0.5)
    ;[1 1 1] Lerp color from healthy to damaged
    (return (`KismetMathLibrary.LinearColorLerp` (`self.ForceFieldDamagedColor`) (`self.ForceFieldHealthyColor`) (/ (- (`local.HealthLevel`) 0.5) 0.5)))
    (else
      ;[1 1 1] Lerp folor from damaged to dead
      (return (`KismetMathLibrary.LinearColorLerp` (`self.ForceFieldDeadColor`) (`self.ForceFieldDamagedColor`) (/ (`local.HealthLevel`) 0.5))))))

(fn `LoseHealth`
  (params (HealthLost :type "Float (double-precision)"))
  (returns (bDied :type Boolean) (ReturnValue :type Boolean))
  (locals (LocalDied :type Boolean :default false))
  (bind _bdepleted (`ResourceComponent.LoseResource` (`self.Health`) HealthLost))
  (set `local.LocalDied` _bdepleted)
  (`MaterialInstanceDynamic.SetVectorParameterValue` (`self.ForceFieldMat`) (`UnicornMaterialParameters.Color`) (`self.GetForceFieldColor`))
  (`|ExecutionSequence`
    (:`then_0`
      (if (`local.LocalDied`)
        (`self.OnShieldBreak`)))
    (:`then_1`
      (`TimelineComponent.SetNewTime` (`self.HealthRegenTimeline`) 0.0)
      (return (`local.LocalDied`) true))))

(fn `UserConstructionScript`
  ;[1 1 1] Get a reference to our forcefield mat so we can adjust it later
  (bind _returnvalue (`KismetMaterialLibrary.CreateDynamicMaterialInstance` "/Game/Unicorn/Spells/M_ForceField.M_ForceField"))
  (bind _output_get (set `self.ForceFieldMat` _returnvalue))
  (`PrimitiveComponent.SetMaterial` (`self.Mesh`) 0 _output_get))