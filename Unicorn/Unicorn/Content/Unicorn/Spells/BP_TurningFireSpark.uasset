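; BP_TurningFireSpark is a fire spark spell projectile that keeps moving forward while gradually curving to the side.
; It caches its initial forward vector on BeginPlay, then yaws around its up axis each tick at YawSpeed.
; Each tick also sets the ProjectileMovement velocity in local space from a weighted blend of initial and current forward, scaled by ProjectileVelocity.X.
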(event `self.ReceiveBeginPlay`
  (`parent.ReceiveBeginPlay`)
  ;[1 1 1] Cache the initial forward vector
  (set `self.InitialForward` (`self.GetActorForwardVector`)))

(event `self.ReceiveTick`
  (params (DeltaSeconds :type "Float (single-precision)"))
  (bind _projectilevelocity_x (`KismetMathLibrary.BreakVector` (`self.ProjectileVelocity`)))
  (`parent.ReceiveTick` DeltaSeconds)
  ;[1 1 1] Rotate around the yaw
  (`self.K2_SetActorRotation` (`KismetMathLibrary.ComposeRotators` (`self.K2_GetActorRotation`) (`KismetMathLibrary.RotatorFromAxisAndAngle` (`self.GetActorUpVector`) (* (`self.YawSpeed`) (`GameplayStatics.GetWorldDeltaSeconds`)))))
  ;[1 1 1] While yawing, update velocity combine a weighted amount of the initial forward vector and the current forward vector, so that we continue to move forward, but also gradually curve to the side
  (`ProjectileMovementComponent.SetVelocityInLocalSpace` (`self.ProjectileMovement`) (* (+ (`KismetMathLibrary.InverseTransformDirection` (`self.GetTransform`) (* (`self.InitialForward`) (`self.VelocityMinInitialForwardPercent`))) (`KismetMathLibrary.MakeVector` (- 1.0 (`self.VelocityMinInitialForwardPercent`)))) _projectilevelocity_x)))

(fn `UserConstructionScript`
  (`parent.UserConstructionScript`))