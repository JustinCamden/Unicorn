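; BP_BossBeam is a boss beam spell that tracks the player while charging, then fires along the locked direction.
; Timers drive the charge, delay, fire and self-destruct stages, with a dynamic material on the cylinder and sphere brightening on firing.
; Actors overlapping at or during firing are hit: destructible ground is destroyed, while other-team actors lose health.
; It reports immunity to projectiles and signals BeamFinished before expiring.
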(event `self.ReceiveBeginPlay`
  (`parent.ReceiveBeginPlay`)
  (`self.ActivateSpell`)
  (set `self.Target` (`GameplayStatics.GetPlayerPawn` 0))
  (`KismetSystemLibrary.K2_SetTimerDelegate` (`|CreateDelegate` :!event `FinishCharging`) (`self.ChargeTime`)))

(event `FinishCharging`
  (set `self.bCharging` false)
  (`KismetSystemLibrary.K2_SetTimerDelegate` (`|CreateDelegate` :!event `FireBeam`) (`self.FireDelay`)))

(event `self.ReceiveTick`
  (params (DeltaSeconds :type "Float (single-precision)"))
  (`parent.ReceiveTick` DeltaSeconds)
  (if (`self.bCharging`)
    (`self.K2_SetActorRotation` (`KismetMathLibrary.FindLookAtRotation` (`self.K2_GetActorLocation`) (`UnicornFunctionLibrary.GetAimLocationOnActor` (`self.Target`))))))

(event `FireBeam`
  (set `self.bFiring` true)
  (`MaterialInstanceDynamic.SetScalarParameterValue` (`self.SpellMat`) (`UnicornMaterialParameters.Emissive`) (`self.FiringEmissive`))
  (`MaterialInstanceDynamic.SetScalarParameterValue` (`self.SpellMat`) (`UnicornMaterialParameters.Opacity`) 1.0)
  (for _array_element (`PrimitiveComponent.GetOverlappingActors` (`self.Cylinder`) null)
    (`self.HitActor` _array_element))
  (`KismetSystemLibrary.K2_SetTimerDelegate` (delegate `SelfDestruct`) (`self.FireTime`)))

(event `self.ReceiveActorBeginOverlap`
  (params (OtherActor :type "Actor Object Reference"))
  (if (`self.bFiring`)
    (`self.HitActor` OtherActor)))

(event `SelfDestruct`
  (`self.BeamFinished`)
  (`self.SetLifeSpan` 0.001))

(fn `HitActor`
  (params (ActorHit :type "Actor Object Reference"))
  (`/Engine/EditorBlueprintResources/StandardMacros.IsValid` ActorHit
    (:`Is Valid`
      (bind _asbp_destructible_ground (cast `/Game/BP_DestructibleGround` ActorHit)
        (:`then`
          (`/Game/BP_DestructibleGround.DestroyGround` _asbp_destructible_ground)
          (return))
        (:`CastFailed`
          (if (not (`TeamComponent.IsSameTeam` (`self.Team`) ActorHit))
            (message `HealthInterface.LoseHealth` (`local.ActorHit`) (`self.DamageAmount`))
            (return)))))))

(fn `ImmuneToPrpjectiles`
  (returns (ReturnValue :type Boolean))
  (return true))

(fn `UserConstructionScript`
  (`parent.UserConstructionScript`)
  (bind _returnvalue (`KismetMaterialLibrary.CreateDynamicMaterialInstance` "/Game/Unicorn/Characters/UnicornCharacter/M_AoEMaterial.M_AoEMaterial"))
  (bind _output_get (set `self.SpellMat` _returnvalue))
  (`PrimitiveComponent.SetMaterial` (`self.Cylinder`) 0 _output_get)
  (`PrimitiveComponent.SetMaterial` (`self.Sphere`) 0 _output_get))