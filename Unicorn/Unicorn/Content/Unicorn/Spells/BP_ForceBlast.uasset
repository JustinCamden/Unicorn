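; BP_ForceBlast is a spell whose cone grows and shrinks on a timeline, damaging each overlapped enemy once before destroying itself.
; On spawn it hits existing overlaps, then optional aim assist turns it by a capped angle toward the enemy best aligned with the desired direction, found by sphere trace.
; If the blast hits no enemy, it spawns an aim-assisted BP_Fireball that inherits its damage, homing and team settings.
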(event `self.ReceiveBeginPlay`
  (`parent.ReceiveBeginPlay`)
  ;[1 1 1] Hit all actors we are already overlapping
  (`self.ActivateSpell`)
  (for _array_element (`self.GetOverlappingActors` null)
    (`self.HitActor` _array_element))
  ;[1 1 1] If aim assisting, rotate to face the best target
  (if (`self.AimAssist`)
    (bind (_success _returnvalue _besttargetaimlocation) (`self.GetBestTarget` (select `bool` (== (`self.DesiredDirection`) (0.0 0.0 0.0)) :`false` (`self.DesiredDirection`) :`true` (`self.GetActorForwardVector`)) (`self.AimAssistAngleTolerance`)))
    (if _success
      (`self.K2_SetActorRotation` (`KismetMathLibrary.RInterpTo_Constant` (`self.K2_GetActorRotation`) (`KismetMathLibrary.FindLookAtRotation` (`self.K2_GetActorLocation`) _besttargetaimlocation) 1.0 (`self.AimAssistMaxAssistAngle`))))))

(event `self.ReceiveActorBeginOverlap`
  (params (OtherActor :type "Actor Object Reference"))
  (`self.HitActor` OtherActor))

(event `self.ReceiveTick`
  (params (DeltaSeconds :type "Float (single-precision)"))
  (`parent.ReceiveTick` DeltaSeconds)
  (switch `/Game/Unicorn/Core/Engine/EGrowthState` (`self.CurrGrowthState`)
    (:`NewEnumerator1`
      (bind (_direction _spheregrowth) (`Timeline|GrowthTimeline` :!label _label)
        (:`Update`
          ;[1 1 1] Handle checking the scale and location of the meshes
          (`SceneComponent.SetRelativeScale3D` (`self.BlastCone`) (`KismetMathLibrary.VLerp` (`self.BlastShrunkSize`) (`self.BlastFullSize`) _spheregrowth)))
        (:`Finished`
          ;[1 1 1] Reverse scaling when finished, and spawn a fireball if we hit nothing
          (switch `ETimelineDirection` _direction
            (:`Forward`
              (set `self.CurrGrowthState` "NewEnumerator2"))
            (:`Backward`
              (`|ExecutionSequence`
                (:`then_0`
                  (if (not (`self.HitEnemy`))
                    (`|SpawnActorFromClass` "/Game/Unicorn/Spells/BP_Fireball.BP_Fireball_C" (`KismetMathLibrary.MakeTransform` (`KismetMathLibrary.TransformLocation` (`self.GetTransform`) (`self.BlastShrunkPosition`)) (`self.K2_GetActorRotation`)) "Undefined" "OverrideRootScale" null (`self.DamageAmount`) (2500.0 0.0 0.0) 3.0 (0.25 0.25 0.25) true (- (`self.AimAssistAngleTolerance`) (`self.AimAssistMaxAssistAngle`)) (`self.GetActorForwardVector`) 1.0 (`self.bHoming`) (`self.HomingRotationSpeed`) (`self.SpellTeam`) (`self.SpellEnemyTeam`) null)))
                (:`then_1`
                  (`self.DeactivateSpell`))))))))
    (:`NewEnumerator2`
      (goto _label :!via `Reverse`))))

(event `self.DeactivateSpell`
  (`parent.DeactivateSpell`)
  (`self.K2_DestroyActor`))

(fn `GetBestTarget`
  (params (DesiredDirection :type "Vector Structure") (AngleTolerance :type "Float (double-precision)" :default 25.0))
  (returns (Success :type Boolean) (ReturnValue :type "Actor Object Reference") (BestTargetAimLocation :type "Vector Structure"))
  (locals (BestTarget :type "Actor Object Reference") (FoundTarget :type Boolean) (BestAimLocation :type "Vector Structure") (CurrTarget :type "Actor Object Reference") (CurrAimLocation :type "Vector Structure") (DirectionToCurrTarget :type "Vector Structure") (CurrTargetScore :type "Float (double-precision)") (BestTargetScore :type "Float (double-precision)" :default -100.0))
  (bind _returnvalue (`self.K2_GetActorLocation`))
  ;[1 1 1] Get all actors within range
  (`|ExecutionSequence`
    (:`then_0`
      (bind (_outhits _returnvalue_2) (`KismetSystemLibrary.SphereTraceMulti` _returnvalue (+ _returnvalue 0.1) (`self.Range`) "TraceTypeQuery1"))
      ;[1 1 1] Filter by enemy actors and valid targets
      (if _returnvalue_2
        (for _array_element _outhits
          (bind _output_get (set `local.CurrTarget` (`.HitActor` (`GameplayStatics.BreakHitResult` _array_element))))
          (`/Engine/EditorBlueprintResources/StandardMacros.IsValid` _output_get
            (:`Is Valid`
              (if (`TeamComponent.IsEnemyTeam` (`self.Team`) _output_get)
                ;[1 1 1] Score and filter targets by angle
                (bind _output_get_2 (set `local.CurrAimLocation` (`UnicornFunctionLibrary.GetAimLocationOnActor` (`local.CurrTarget`) (`self.VRAimLocationHeightMultiplier`))))
                (bind _output_get_3 (set `local.DirectionToCurrTarget` (`KismetMathLibrary.Normal` (- _output_get_2 (`self.K2_GetActorLocation`)))))
                (bind _output_get_4 (set `local.CurrTargetScore` (`KismetMathLibrary.Dot_VectorVector` _output_get_3 (`local.DesiredDirection`))))
                (if (and (>= _output_get_4 (`KismetMathLibrary.DegCos` (`local.AngleTolerance`))) (> (`local.CurrTargetScore`) (`local.BestTargetScore`)))
                  (set `local.BestTarget` (`local.CurrTarget`))
                  (set `local.BestTargetScore` (`local.CurrTargetScore`))
                  (set `local.BestAimLocation` (`local.CurrAimLocation`))
                  (set `local.FoundTarget` true))))))))
    (:`then_1`
      (return (`local.FoundTarget`) (`local.BestTarget`) (`local.BestAimLocation`)))))

(fn `HitActor`
  (params (HitActor :type "Actor Object Reference"))
  (`|ExecutionSequence`
    (:`then_0`
      (if (`self.bSpellActive`)
        (if (`TeamComponent.IsEnemyTeam` (`self.Team`) (`local.HitActor`))
          (if (not (`KismetArrayLibrary.Array_Contains` (`self.HitActors`) (`local.HitActor`)))
            (`KismetArrayLibrary.Array_Add` (`self.HitActors`) (`local.HitActor`))
            (message `HealthInterface.LoseHealth` (`local.HitActor`) (`self.DamageAmount`))
            (set `self.HitEnemy` true)))))
    (:`then_1`
      (return))))

(fn `UserConstructionScript`
  (`parent.UserConstructionScript`))