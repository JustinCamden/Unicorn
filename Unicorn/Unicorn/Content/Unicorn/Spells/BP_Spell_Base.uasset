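; BP_Spell_Base is a base actor for spells, providing team setup and an on/off active state.
; The construction script copies the spell's team and enemy team into its Team component.
; ActivateSpell and DeactivateSpell set the SpellActive flag, and Safe variants call them only when the state would change.
; The event graph holds only empty placeholder events, so the base has no runtime behavior of its own.
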(event `self.ReceiveBeginPlay`)

(fn `ActivateSpell`
  (set `self.bSpellActive` true)
  (return))

(fn `DeactivateSpell`
  (set `self.bSpellActive` false)
  (return))

(fn `SafeActivateSpell`
  (if (not (`self.bSpellActive`))
    (`self.ActivateSpell`)
    (return)))

(fn `SafeDeactivateSpell`
  (if (`self.bSpellActive`)
    (`self.DeactivateSpell`)
    (return)))

(fn `UserConstructionScript`
  ;[1 1 1] Initialize team on construct
  (set `TeamComponent.Team` (`self.SpellTeam`) (`self.Team`))
  (set `TeamComponent.EnemyTeam` (`self.SpellEnemyTeam`) (`self.Team`)))