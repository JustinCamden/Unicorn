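; BP_Forcefield is a spell forcefield with health, shown as a sphere that changes color with damage.
; Construction gives the sphere a dynamic material set to HealthyColor.
; LoseHealth drains the Health resource and lerps HealthyColor toward DamagedColor by current/max health, though that write targets parameter "None" and the ratio runs inverted.
; Losing all health triggers a short lifespan, while GainHealth always returns false.
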(fn `Die`
  (`self.SetLifeSpan` 0.1))

(fn `GainHealth`
  (params (HealthGained :type "Float (double-precision)"))
  (returns (ReturnValue :type Boolean))
  (return false))

(fn `LoseHealth`
  (params (HealthLost :type "Float (double-precision)"))
  (returns (bDied :type Boolean) (ReturnValue :type Boolean))
  (bind _health (`self.Health`))
  ;[1 1 1] Update health and color
  (bind _bdepleted (`ResourceComponent.LoseResource` (`self.Health`) HealthLost))
  (`MaterialInstanceDynamic.SetVectorParameterValue` (`self.ForceFieldMaterial`) "None" (`KismetMathLibrary.LinearColorLerp` (`self.HealthyColor`) (`self.DamagedColor`) (/ (`ResourceComponent.CurrentResource` _health) (`ResourceComponent.MaxResource` _health))))
  ;[1 1 1] Die upon losing all health
  (if _bdepleted
    (`self.Die`))
  (return _bdepleted true))

(fn `UserConstructionScript`
  (bind _returnvalue (`KismetMaterialLibrary.CreateDynamicMaterialInstance` "/Game/Unicorn/Spells/M_ForceField.M_ForceField"))
  (bind _output_get (set `self.ForceFieldMaterial` _returnvalue))
  (`MaterialInstanceDynamic.SetVectorParameterValue` _output_get (`UnicornMaterialParameters.Color`) (`self.HealthyColor`))
  (`PrimitiveComponent.SetMaterial` (`self.Sphere`) 0 (`self.ForceFieldMaterial`)))