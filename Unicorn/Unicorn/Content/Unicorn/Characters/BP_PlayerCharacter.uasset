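; Player character Blueprint that manages health, damage, death and a damage screen effect.
; A Health resource handles gain and loss, and depletion calls Die, which only sets the Dead flag.
; Tick plays a timeline that scales health regen and drives the damage post-process weight through interpolation, while each hit rewinds it to zero.
; The mana regen effect check on Tick is a stub with no resulting action.
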(event `self.ReceiveBeginPlay`
  (`PostProcessComponent.AddOrUpdateBlendable` (`self.HUDPostProcess`) (`self.DamagePPEffect`) 0.0))

(event `self.ReceiveTick`
  (params (DeltaSeconds :type "Float (single-precision)"))
  (`|ExecutionSequence`
    (:`then_0`
      (if (not (and (`ResourceComponent.IsAtMaxCapacity` (`self.Health`)) (> (`self.CurrDamagePPWeight`) 0.0)))
        (bind (_direction _percentmaxhealthregen _damageppeffect) (`Timeline|HealthRegenTimeline`)
          (:`Update`
            (`ResourceComponent.GainResource` (`self.Health`) (* _percentmaxhealthregen (`self.MaxHealthRegenPerSec`)))
            (bind _output_get (set `self.CurrDamagePPWeight` (`KismetMathLibrary.FInterpTo` (`self.CurrDamagePPWeight`) _damageppeffect (`GameplayStatics.GetWorldDeltaSeconds`) (`self.PPLerpSpeed`))))
            (`PostProcessComponent.AddOrUpdateBlendable` (`self.HUDPostProcess`) (`self.DamagePPEffect`) _output_get)))))
    (:`then_1`
      ;[1 1 1] Check whether the mana regen PP is showing
      (if (> (`self.CurrManaRegenPPWeight`) 0.0)
        (if (`ResourceComponent.IsAtMaxCapacity` (`self.Mana`))
          _)))))

(fn `Die`
  (set `self.bDead` true)
  (return))

(fn `GainHealth`
  (params (HealthGained :type "Float (double-precision)"))
  (returns (ReturnValue :type Boolean))
  (`ResourceComponent.GainResource` (`self.Health`) HealthGained)
  (return true))

(fn `LoseHealth`
  (params (HealthLost :type "Float (double-precision)"))
  (returns (bDied :type Boolean) (ReturnValue :type Boolean))
  (`|ExecutionSequence`
    (:`then_0`
      ;[1 1 1] Only lose health if we are dead
      (if (not (`self.bDead`))
        ;[1 1 1] Update damage timeline, lose health and call die on health depleted
        (`TimelineComponent.SetNewTime` (`self.HealthRegenTimeline`) 0.0)
        (bind _bdepleted (`ResourceComponent.LoseResource` (`self.Health`) HealthLost))
        (if _bdepleted
          (`self.Die`)
          (return true true)
          (else
            (return false true)))))
    (:`then_1`
      (return false false))))

(fn `UserConstructionScript`)