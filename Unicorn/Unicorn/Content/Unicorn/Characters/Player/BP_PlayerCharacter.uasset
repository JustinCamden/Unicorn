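; VR player character that casts fireballs with punch gestures and teleports along a projected arc.
; Tick drives health and mana regen, a teleport state machine, and per-hand punch detection from kinematic tracker velocity and travel distance.
; Timelines drive regen rates and post-process material opacity for damage, mana regen and teleport blackout.
; Teleport checks mana without spending it; the left punch's affordability check uses zero instead of the spell cost.
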(event `self.ReceiveBeginPlay`
  ;[1 1 1] Add blendables to the PP volume
  (`PostProcessComponent.AddOrUpdateBlendable` (`self.HUDPostProcess`) (`self.DamagePPMaterial`) 1.0)
  (`PostProcessComponent.AddOrUpdateBlendable` (`self.HUDPostProcess`) (`self.ManaRegenPPEffect`) 1.0)
  (`PostProcessComponent.AddOrUpdateBlendable` (`self.HUDPostProcess`) (`self.BlackoutPPMaterial`) 1.0)
  ;[1 1 1] Update widget
  (bind _asbp_player_stats_ui (cast `/Game/Unicorn/Characters/Player/BP_PlayerStats_UI` (`WidgetComponent.GetUserWidgetObject` (`self.HUDWidget`))))
  (set `/Game/Unicorn/Characters/Player/BP_PlayerStats_UI.OwningPlayerCharacter` self _asbp_player_stats_ui)
  (`/Game/Unicorn/Core/Engine/BP_KinematicVelocity_Component.ActivateKinematicTracking` (`self.RightKinematicTracker`))
  (`/Game/Unicorn/Core/Engine/BP_KinematicVelocity_Component.ActivateKinematicTracking` (`self.LeftKinematicTracker`)))

(event `self.ReceiveTick`
  (params (DeltaSeconds :type "Float (single-precision)"))
  (bind _rightmotioncontroller (`self.RightMotionController`))
  (bind _leftkinematictracker (`self.LeftKinematicTracker`))
  (bind _rightkinematictracker (`self.RightKinematicTracker`))
  (bind _leftkinematictracker_2 (`self.LeftKinematicTracker`))
  (bind _rightkinematictracker_2 (`self.RightKinematicTracker`))
  (`|ExecutionSequence`
    (:`then_0`
      (if (not (and (`ResourceComponent.IsAtMaxCapacity` (`self.Health`)) (<= (`self.CurrDamagePPWeight`) 0.0)))
        (bind (_direction _percentmaxhealthregen _damageppblendweight) (`Timeline|HealthRegenTimeline`)
          (:`Update`
            (`ResourceComponent.GainResource` (`self.Health`) (* _percentmaxhealthregen (`self.MaxHealthRegenPerSec`)))
            (bind _output_get (set `self.CurrDamagePPWeight` (`KismetMathLibrary.FInterpTo` (`self.CurrDamagePPWeight`) _damageppblendweight (`GameplayStatics.GetWorldDeltaSeconds`) (`self.PPLerpSpeed`))))
            (`MaterialInstanceDynamic.SetScalarParameterValue` (`self.DamagePPMaterial`) (`UnicornMaterialParameters.Opacity`) _output_get)))))
    (:`then_1`
      (if (`ResourceComponent.IsAtMaxCapacity` (`self.Mana`))
        (if (not (<= (`self.CurrManaRegenPPWeight`) 0.0))
          (bind (_direction_2 _percentmaxmanaregen _manaregenppblendweight) (`Timeline|ManaRegenTimeline` :!via `Reverse` :!label _label)
            (:`Update`
              (`ResourceComponent.GainResource` (`self.Mana`) (* (`self.MaxManaRegenPerSecond`) _percentmaxmanaregen))
              (bind _output_get_2 (set `self.CurrManaRegenPPWeight` (`KismetMathLibrary.FInterpTo` (`self.CurrManaRegenPPWeight`) _manaregenppblendweight (`GameplayStatics.GetWorldDeltaSeconds`) (`self.PPLerpSpeed`))))
              (`MaterialInstanceDynamic.SetScalarParameterValue` (`self.ManaRegenPPEffect`) (`UnicornMaterialParameters.Opacity`) _output_get_2))))
        (else
          (goto _label))))
    (:`then_2`
      (switch `/Game/Unicorn/Core/Engine/ETeleportState` (`self.CurrTeleportState`)
        (:`NewEnumerator3`
          (if (`|EnumEquality` (`self.CurrTeleportState`) "NewEnumerator3")
            (`self.TraceTeleportLocation` (`SceneComponent.K2_GetComponentLocation` _rightmotioncontroller) (`SceneComponent.GetForwardVector` _rightmotioncontroller) (`self.TeleportTraceSpeed`))
            (else
              (set `self.CurrTeleportState` "NewEnumerator0"))))
        (:`NewEnumerator1`
          (bind (_direction_3 _blackoutweight) (`Timeline|TeleportTimeline` :!label _label_2)
            (:`Update`
              (`MaterialInstanceDynamic.SetScalarParameterValue` (`self.BlackoutPPMaterial`) "Opacity" _blackoutweight))
            (:`Finished`
              (if (`|EnumEquality` (`self.CurrTeleportState`) "NewEnumerator1")
                (`VRBaseCharacterMovementComponent.PerformMoveAction_Teleport` (`self.VRMovementReference`) (`self.GetTeleportLocation` (`self.TeleportLocation`)) (`self.K2_GetActorRotation`))
                (set `self.CurrTeleportState` "NewEnumerator2")
                (else
                  (set `self.CurrTeleportState` "NewEnumerator0"))))))
        (:`NewEnumerator2`
          (goto _label_2 :!via `Reverse`))))
    (:`then_3`
      (`|ExecutionSequence`
        (:`then_0`
          (bind (_outdrawinglinesegment _outlinesegmentlength _successfullyfinishedsegment) (`self.CheckCompletedLineSegment` (`self.bPunchingRight`) (`self.CurrPunchLengthRight`) (`SceneComponent.GetForwardVector` _rightkinematictracker) (`self.PunchVelocityMin`) (`self.PunchVelocityDotMin`) (`self.PunchLengthMin`) _rightkinematictracker))
          (set `self.bPunchingRight` _outdrawinglinesegment)
          (set `self.CurrPunchLengthRight` _outlinesegmentlength)
          (if _successfullyfinishedsegment
            (if (`ResourceComponent.CanAfford` (`self.Mana`) (`self.PunchSpellCost`))
              (`self.SpendMana` (`self.PunchSpellCost`))
              (`|SpawnActorFromClass` "/Game/Unicorn/Spells/Fireball_Spell.Fireball_Spell_C" (`KismetMathLibrary.MakeTransform` (`SceneComponent.K2_GetComponentLocation` _rightkinematictracker_2) (`SceneComponent.K2_GetComponentRotation` _rightkinematictracker_2)) "Undefined" "OverrideRootScale" null 10.0 (1000.0 0.0 0.0) null))))
        (:`then_1`
          (bind (_outdrawinglinesegment_2 _outlinesegmentlength_2 _successfullyfinishedsegment_2) (`self.CheckCompletedLineSegment` (`self.bPunchingLeft`) (`self.CurrPunchLengthLeft`) (`SceneComponent.GetForwardVector` _leftkinematictracker) (`self.PunchVelocityMin`) (`self.PunchVelocityDotMin`) (`self.PunchLengthMin`) _leftkinematictracker))
          (set `self.bPunchingLeft` _outdrawinglinesegment_2)
          (set `self.CurrPunchLengthLeft` _outlinesegmentlength_2)
          (if _successfullyfinishedsegment_2
            (if (`ResourceComponent.CanAfford` (`self.Mana`) 0.0)
              (`self.SpendMana` (`self.PunchSpellCost`))
              (`|SpawnActorFromClass` "/Game/Unicorn/Spells/Fireball_Spell.Fireball_Spell_C" (`KismetMathLibrary.MakeTransform` (`SceneComponent.K2_GetComponentLocation` _leftkinematictracker_2) (`SceneComponent.K2_GetComponentRotation` _leftkinematictracker_2)) "Undefined" "OverrideRootScale" null 10.0 (1000.0 0.0 0.0) null))))))))

(event `InputAction|TeleportRight`
  (params (Key :type "Key Structure"))
  (bind _rightmotioncontroller (`self.RightMotionController`))
  (:`Pressed`
    (if (and (`|EnumEquality` (`self.CurrTeleportState`) "NewEnumerator0") (`ResourceComponent.CanAfford` (`self.Mana`) (`self.TeleportCost`)))
      (set `self.CurrTeleportState` "NewEnumerator3")))
  (:`Released`
    (if (`|EnumEquality` (`self.CurrTeleportState`) "NewEnumerator3")
      (if (`ResourceComponent.CanAfford` (`self.Mana`) (`self.TeleportCost`))
        (bind (_teleportlocation _success) (`self.TraceTeleportLocation` (`SceneComponent.K2_GetComponentLocation` _rightmotioncontroller) (`SceneComponent.GetForwardVector` _rightmotioncontroller) (`self.TeleportTraceSpeed`)))
        (if _success
          (set `self.TeleportLocation` _teleportlocation)
          (set `self.CurrTeleportState` "NewEnumerator1")
          (else
            (set `self.CurrTeleportState` "NewEnumerator0")))
        (else
          (set `self.CurrTeleportState` "NewEnumerator0"))))))

(fn `CheckCompletedLineSegment`
  (params (CurrDrawingLineSegment :type Boolean) (CurrLineSegmentLength :type "Float (double-precision)") (LineSegmentAngle :type "Vector Structure") (MinLineSegmentVelocity :type "Float (double-precision)") (MinLineSegmentVelocityDot :type "Float (double-precision)") (MinLineSegmentLength :type "Float (double-precision)") (KinematicTracker :type "/Game/Unicorn/Core/Engine/BP_KinematicVelocity_Component Object Reference"))
  (returns (OutDrawingLineSegment :type Boolean) (OutLineSegmentLength :type "Float (double-precision)") (SuccessfullyFinishedSegment :type Boolean))
  (locals (bWasDrawingLineSegment :type Boolean) (bLocalDrawingLineSegment :type Boolean) (LocalLineSegmentLength :type "Float (double-precision)") (LocalLineSegmentAngle :type "Vector Structure") (bLineFinished :type Boolean))
  (`|ExecutionSequence`
    (:`then_0`
      ;[1 1 1] Update local variables
      (set `local.bWasDrawingLineSegment` (`local.CurrDrawingLineSegment`))
      (set `local.LocalLineSegmentAngle` (`KismetMathLibrary.Normal` (`local.LineSegmentAngle`)))
      (set `local.LocalLineSegmentLength` (`local.CurrLineSegmentLength`))
      ;[1 1 1] Get whether we are moving in the direction of the linesegment at at least the minimum velocity
      (bind (_returnvalue _returnvaluenormalized) (`/Game/Unicorn/Core/Engine/BP_KinematicVelocity_Component.GetVelocityAlongAngle` (`local.KinematicTracker`) (`local.LineSegmentAngle`)))
      (bind _output_get (set `local.bLocalDrawingLineSegment` (and (>= _returnvalue (`local.MinLineSegmentVelocity`)) (>= _returnvaluenormalized (`local.MinLineSegmentVelocityDot`)))))
      ;[1 1 1] If we are, then update the current line length by the distance we have traveled in the line's direction
      (if _output_get
        (set `local.LocalLineSegmentLength` (+ (`local.CurrLineSegmentLength`) (`/Game/Unicorn/Core/Engine/BP_KinematicVelocity_Component.GetAngularDeltaPosition` (`local.KinematicTracker`) (`local.LineSegmentAngle`))))
        (else
          ;[1 1 1] If not, but we were previously, check whether we reached the minimum line segment length
          (if (`local.bWasDrawingLineSegment`)
            (set `local.bLineFinished` (>= (`local.LocalLineSegmentLength`) (`local.MinLineSegmentLength`)))
            (set `local.LocalLineSegmentLength` 0.0)))))
    (:`then_1`
      (return (`local.bLocalDrawingLineSegment`) (`local.LocalLineSegmentLength`) (`local.bLineFinished`)))))

(fn `Die`
  (set `self.bDead` true)
  (return))

(fn `GainHealth`
  (params (HealthGained :type "Float (double-precision)"))
  (returns (ReturnValue :type Boolean))
  (`ResourceComponent.GainResource` (`self.Health`) HealthGained)
  (return true))

(fn `LoseHealth`
  (params (HealthLost :type "Float (double-precision)"))
  (returns (bDied :type Boolean) (ReturnValue :type Boolean))
  (`|ExecutionSequence`
    (:`then_0`
      ;[1 1 1] Only lose health if we are dead
      (if (not (`self.bDead`))
        ;[1 1 1] Update damage timeline, lose health and call die on health depleted
        (`TimelineComponent.SetNewTime` (`self.HealthRegenTimeline`) 0.0)
        (bind _bdepleted (`ResourceComponent.LoseResource` (`self.Health`) HealthLost))
        (if _bdepleted
          (`self.Die`)
          (return true true)
          (else
            (return false true)))))
    (:`then_1`
      (return false false))))

(fn `SpendMana`
  (params (AmountToSpend :type "Float (double-precision)"))
  ;[1 1 1] Lose mana resource and reset the regen timeline
  (`ResourceComponent.LoseResource` (`self.Mana`) AmountToSpend)
  (`TimelineComponent.SetNewTime` (`self.ManaRegenTimeline`) 0.0)
  (return))

(fn `TraceTeleportLocation`
  (params (StartingLocation :type "Vector Structure") (ForwardVector :type "Vector Structure") (Speed :type "Float (double-precision)"))
  (returns (TeleportLocation :type "Vector Structure") (Success :type Boolean))
  (locals (LocalTeleportLocation :type "Vector Structure"))
  (bind (_localteleportlocation_x _localteleportlocation_y _localteleportlocation_z) (`KismetMathLibrary.BreakVector` (`local.LocalTeleportLocation`)))
  (bind (_localteleportlocation_x_2 _localteleportlocation_y_2 _localteleportlocation_z_2) (`KismetMathLibrary.BreakVector` (`local.LocalTeleportLocation`)))
  ;[1 1 1] Predict path along the inputted starting location, forward vector, and velocity
  (bind (_outhit _outpathpositions _outlasttracedestination _returnvalue) (`GameplayStatics.Blueprint_PredictProjectilePath_ByTraceChannel` StartingLocation (* ForwardVector Speed) true 0.0 "ECC_WorldStatic" false (`|MakeArray` self :!type "Actor Object Reference") "ForOneFrame"))
  (bind (_projectedlocation _returnvalue_2) (`NavigationSystem.K2_ProjectPointToNavigation` (`.Location` (`GameplayStatics.BreakHitResult` _outhit))))
  ;[1 1 1] Check if we hit a point and its on the navigation system
  (set `local.LocalTeleportLocation` _projectedlocation)
  (if (and _returnvalue_2 _returnvalue)
    ;[1 1 1] Draw debug cylinders and return whether we successfully traced or not
    (`KismetSystemLibrary.DrawDebugCylinder` (`local.LocalTeleportLocation`) (`KismetMathLibrary.MakeVector` _localteleportlocation_x_2 _localteleportlocation_y_2 (+ _localteleportlocation_z_2 20.0)) 20.0 12 (struct :`G` 1.0 :`B` 0.0425 :`A` 1.0))
    (return (`local.LocalTeleportLocation`) true)
    (else
      (`KismetSystemLibrary.DrawDebugCylinder` (`local.LocalTeleportLocation`) (`KismetMathLibrary.MakeVector` _localteleportlocation_x _localteleportlocation_y (+ _localteleportlocation_z 20.0)) 20.0 12 (struct :`R` 1.0 :`B` 0.039766 :`A` 1.0))
      (return (0.0 0.0 0.0) false))))

(fn `UserConstructionScript`
  (`|ExecutionSequence`
    (:`then_0`
      ;[1 1 1] Initialize material instances
      (bind _returnvalue (`KismetMaterialLibrary.CreateDynamicMaterialInstance` "/Game/Unicorn/Core/MaterialLibrary/MI_BlackoutPP.MI_BlackoutPP"))
      (bind _output_get (set `self.BlackoutPPMaterial` _returnvalue))
      (`MaterialInstanceDynamic.SetScalarParameterValue` _output_get (`UnicornMaterialParameters.Opacity`) 0.0))
    (:`then_1`
      (bind _returnvalue_2 (`KismetMaterialLibrary.CreateDynamicMaterialInstance` "/Game/Unicorn/Core/MaterialLibrary/MI_DamagePP.MI_DamagePP"))
      (bind _output_get_2 (set `self.DamagePPMaterial` _returnvalue_2))
      (`MaterialInstanceDynamic.SetScalarParameterValue` _output_get_2 (`UnicornMaterialParameters.Opacity`) 0.0))
    (:`then_2`
      (bind _returnvalue_3 (`KismetMaterialLibrary.CreateDynamicMaterialInstance` "/Game/Unicorn/Core/MaterialLibrary/MI_ManaRegenPP.MI_ManaRegenPP"))
      (bind _output_get_3 (set `self.ManaRegenPPEffect` _returnvalue_3))
      (`MaterialInstanceDynamic.SetScalarParameterValue` _output_get_3 (`UnicornMaterialParameters.Opacity`) 0.0))))