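; An actor that serves as a floating UI anchor in front of the owning VR character's camera.
; Each tick it eases toward a point at a set view distance from the camera and rotates to face it.
; The target direction uses clamped camera pitch, or zero with vertical lock.
; Its yaw comes from the camera when horizontal lock is on, otherwise from the character actor.
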(event `self.ReceiveTick`
  (params (DeltaSeconds :type "Float (single-precision)"))
  (`self.K2_SetActorLocationAndRotation` (`KismetMathLibrary.VInterpTo` (`self.K2_GetActorLocation`) (`self.GetViewLocation`) (`GameplayStatics.GetWorldDeltaSeconds`) (`self.RotationSpeed`)) (`self.GetViewRotation`)))

(fn `GetViewLocation`
  (returns (ReturnValue :type "Vector Structure"))
  (bind _owningvrcharacter (`self.OwningVRCharacter`))
  (bind (_returnvalue_roll _returnvalue_pitch _returnvalue_yaw) (`KismetMathLibrary.BreakRotator` (`self.K2_GetActorRotation` _owningvrcharacter)))
  (bind (_returnvalue_roll_2 _returnvalue_pitch_2 _returnvalue_yaw_2) (`KismetMathLibrary.BreakRotator` (`SceneComponent.K2_GetComponentRotation` (`VRBaseCharacter.VRReplicatedCamera` _owningvrcharacter))))
  (return (+ (* (`KismetMathLibrary.GetForwardVector` (`KismetMathLibrary.MakeRotator` _returnvalue_roll_2 (select `bool` (`self.LockVerticalRotation`) :`false` (`KismetMathLibrary.FClamp` _returnvalue_pitch_2 (`self.PitchMin`) (`self.PitchMax`))) (select `bool` (`self.LockHorizontalRotation`) :`false` _returnvalue_yaw :`true` _returnvalue_yaw_2))) (`self.ViewDistance`)) (`SceneComponent.K2_GetComponentLocation` (`VRBaseCharacter.VRReplicatedCamera` (`self.OwningVRCharacter`))))))

(fn `GetViewRotation`
  (returns (ReturnValue :type "Rotator Structure"))
  (return (`KismetMathLibrary.FindLookAtRotation` (`self.K2_GetActorLocation`) (`SceneComponent.K2_GetComponentLocation` (`VRBaseCharacter.VRReplicatedCamera` (`self.OwningVRCharacter`))))))

(fn `UserConstructionScript`)