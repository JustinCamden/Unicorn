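; BP_CapsuleCharacter is a simple team-based capsule character with health, stun, knockback and stand-in melee and ranged attacks.
; Construction sets its teams and a tinted dynamic material.
; Attacks only start fixed-delay timers, with events that send attack-finished notifications.
; Losing health plays a sound and sets a Hurt flag that Tick uses to run a color-flash timeline, while death destroys the actor after parent handling.
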(event `OnRangedAttackFinished`
  (`self.NotifyRangedAttackFinished`))

(event `OnMeleeAttackFinished`
  (`self.NotifyMeleeAttackFinished`))

(event `self.ReceiveBeginPlay`)

(event `self.OnDeath`
  (`parent.OnDeath`)
  (`self.K2_DestroyActor`))

(event `self.ReceiveTick`
  (params (DeltaSeconds :type "Float (single-precision)"))
  ;[1 1 1] If we are hurt, then play the hurt color timeline forward, then backward, to signal that the character was hit
  (if (`self.bHurt`)
    (bind (_direction _percenthurtcolor) (`Timeline|HurtColorTimeline`)
      (:`Update`
        (`MaterialInstanceDynamic.SetVectorParameterValue` (`self.BodyMat`) (`UnicornMaterialParameters.Color`) (`KismetMathLibrary.LinearColorLerp` (`self.BodyColor`) (`self.HurtColor`) _percenthurtcolor)))
      (:`Finished`
        (set `self.bHurt` false)))))

(fn `BeStunned`
  (params (StunPower :type "/Game/Unicorn/Core/Engine/EPowerLevel Enum" :default "NewEnumerator0"))
  (returns (Success :type Boolean))
  (`/Game/Unicorn/Core/Engine/BP_StunComponent.Stun` (`self.BP_StunComponent`) StunPower)
  (return true))

(fn `DoMeleeAttack`
  (`KismetSystemLibrary.K2_ClearAndInvalidateTimerHandle` (`self.MeleeAttackTimer`))
  (bind _returnvalue (`KismetSystemLibrary.K2_SetTimerDelegate` (`|CreateDelegate` :!event `OnMeleeAttackFinished`) 3.0))
  (set `self.MeleeAttackTimer` _returnvalue)
  (return))

(fn `DoRangedAttack`
  (`KismetSystemLibrary.K2_ClearAndInvalidateTimerHandle` (`self.RangedAttackTimer`))
  (bind _returnvalue (`KismetSystemLibrary.K2_SetTimerDelegate` (`|CreateDelegate` :!event `OnRangedAttackFinished`) 3.0))
  (set `self.RangedAttackTimer` _returnvalue)
  (return))

(fn `GetCapsuleController`
  (returns (ReturnValue :type "UnicornAIController Object Reference"))
  (bind _asbp_capsule_controller (cast `/Game/Unicorn/Characters/UnicornCharacter/BP_CapsuleController` (`self.GetController`)))
  (return _asbp_capsule_controller))

(fn `GetVisionComponent`
  (returns (ReturnValue :type "SceneComponent Object Reference"))
  (return (`self.Vision`)))

(fn `Knockback`
  (params (KnockbackOrigin :type "Vector Structure") (VelocityMagnitude :type "Float (double-precision)"))
  (returns (Success :type Boolean))
  (`self.LaunchCharacter` (* (`KismetMathLibrary.Normal` (`/Game/Unicorn/Core/Engine/BPFL_UnicornLibrary.FlattenZ` (- (`self.K2_GetActorLocation`) KnockbackOrigin))) VelocityMagnitude))
  (`self.NotifyKnockedBack`)
  (return true))

(fn `LoseHealth`
  (params (HealthLost :type "Float (double-precision)"))
  (returns (bDied :type Boolean) (ReturnValue :type Boolean))
  (`GameplayStatics.SpawnSoundAttached` "/Game/ProSoundCollection_v1_3/Footsteps/Cues/footstep_ice_crunchy_land_01_Cue.footstep_ice_crunchy_land_01_Cue" (`self.RootComponent`) "None" (0.0 0.0 0.0) (struct) "KeepRelativeOffset" false 1.0 1.0 0.0 "/Game/ATT_Spell.ATT_Spell" "/Game/CON_Spell.CON_Spell")
  (bind (_bdied _returnvalue) (`parent.LoseHealth` HealthLost))
  (set `self.bHurt` true)
  (return _bdied _returnvalue))

(fn `UserConstructionScript`
  (set `TeamComponent.Team` (`self.Team`) (`self.TeamComponent`))
  (set `TeamComponent.EnemyTeam` (`self.EnemyTeam`) (`self.TeamComponent`))
  (bind _returnvalue (`KismetMaterialLibrary.CreateDynamicMaterialInstance` "/Game/Unicorn/Characters/UnicornCharacter/M_CapsuleMaterial.M_CapsuleMaterial"))
  (bind _output_get (set `self.BodyMat` _returnvalue))
  (`MaterialInstanceDynamic.SetVectorParameterValue` _output_get (`UnicornMaterialParameters.Color`) (`self.BodyColor`))
  (`PrimitiveComponent.SetMaterial` (`self.Sphere`) 0 (`self.BodyMat`)))