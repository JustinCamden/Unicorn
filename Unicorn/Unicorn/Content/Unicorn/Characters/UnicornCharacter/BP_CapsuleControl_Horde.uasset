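; AI controller for a Horde capsule character that starts the BT_Capsule_Melee behavior tree on BeginPlay.
; When a melee attack finishes, it raises a recently-attacked flag and restarts a one-shot timer, provided the configured duration is positive.
; A timer-finished handler clears the flag.
; The node binding the attack-finished notification is disconnected, so this graph does not register that handler itself.
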(event `self.ReceiveBeginPlay`
  (`parent.ReceiveBeginPlay`)
  (`self.RunBehaviorTree` "/Game/Unicorn/Characters/UnicornCharacter/BT_Capsule_Melee.BT_Capsule_Melee"))

(event `self.ReceiveTick`
  (params (DeltaSeconds :type "Float (single-precision)"))
  (`parent.ReceiveTick` DeltaSeconds))

(event `OnMeleeAttackFinished`
  (if (> (`self.RecentlyAttackedTimerTime`) 0.0)
    (`KismetSystemLibrary.K2_ClearAndInvalidateTimerHandle` (`self.RecentlyAttackedTimer`))
    (set `self.bRecentlyCompletedMeleeAttack` true)
    (bind _returnvalue (`KismetSystemLibrary.K2_SetTimerDelegate` (`|CreateDelegate` :!event `OnMeleeAttackTimerFinished`) (`self.RecentlyAttackedTimerTime`)))
    (set `self.RecentlyAttackedTimer` _returnvalue)))

(event `OnMeleeAttackTimerFinished`
  (set `self.bRecentlyCompletedMeleeAttack` false))

(fn `UserConstructionScript`
  (`parent.UserConstructionScript`))