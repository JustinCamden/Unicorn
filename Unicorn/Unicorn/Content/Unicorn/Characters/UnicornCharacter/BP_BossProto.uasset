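; Prototype boss character with melee AoE, ice spike and beam attacks, plus shield- and state-based invincibility.
; Boss state lives on BP_CapsuleCon_Boss; death in Normal activates a power pillar, or moves the boss to a stationary phase when none remain.
; Tick-driven timelines handle charge growth with health refill, shrinking and that move.
; Hitbox swing code remains, but MeleeAttack returns before reaching it, spawning BT_BossAoE instead.
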(event `self.ReceiveBeginPlay`
  (`self.SetShield` true)
  (`parent.ReceiveBeginPlay`)
  (set `self.NormalSize` (`self.GetActorScale3D`)))

(event `self.HitboxRight.OnComponentBeginOverlap`
  (params (OverlappedComponent :type "PrimitiveComponent Object Reference") (OtherActor :type "Actor Object Reference") (OtherComp :type "PrimitiveComponent Object Reference") (OtherBodyIndex :type Integer) (bFromSweep :type Boolean) (SweepResult :type "HitResult Structure (by ref)"))
  (if (`|EnumEquality` (`self.AttackStateRight`) "NewEnumerator0")
    (`self.HitActor` OtherActor)))

(event `self.HitboxLeft.OnComponentBeginOverlap`
  (params (OverlappedComponent :type "PrimitiveComponent Object Reference") (OtherActor :type "Actor Object Reference") (OtherComp :type "PrimitiveComponent Object Reference") (OtherBodyIndex :type Integer) (bFromSweep :type Boolean) (SweepResult :type "HitResult Structure (by ref)"))
  (if (`|EnumEquality` (`self.AttackStateLeft`) "NewEnumerator2")
    (`self.HitActor` OtherActor)))

(event `self.ReceiveTick`
  (params (DeltaSeconds :type "Float (single-precision)"))
  (bind _returnvalue (`self.GetBossCon`))
  (bind _healthcomponent (`self.HealthComponent`))
  (`parent.ReceiveTick` DeltaSeconds)
  (`|ExecutionSequence`
    (:`then_0`
      (if (not (`self.bDead`))
        (`|ExecutionSequence`
          (:`then_0`
            (switch `/Game/Unicorn/Core/Engine/EAttackState` (`self.AttackStateLeft`)
              (:`NewEnumerator0`
                (bind (_direction _attacklefttime) (`Timeline|AttackLeftTimeline` :!label _label)
                  (:`Update`
                    (`SceneComponent.K2_SetRelativeLocation` (`self.HitboxLeft`) (`KismetMathLibrary.VLerp` (`self.HitboxPositionInactiveLeft`) (`self.HitboxPositionActiveLeft`) _attacklefttime) false false)
                    (`SceneComponent.SetRelativeScale3D` (`self.HitboxLeft`) (`KismetMathLibrary.VLerp` (`self.HitboxLocalScaleInactive`) (`self.HitboxLocalScaleActive`) _attacklefttime)))
                  (:`Finished`
                    (switch `ETimelineDirection` _direction
                      (:`Forward`
                        (set `self.AttackStateLeft` "NewEnumerator1"))
                      (:`Backward`
                        (set `self.AttackStateLeft` "NewEnumerator2")
                        (`self.OnMeleeAttackFinishedLeft`))))))
              (:`NewEnumerator1`
                (goto _label :!via `Reverse`))))
          (:`then_1`
            (switch `/Game/Unicorn/Core/Engine/EAttackState` (`self.AttackStateRight`)
              (:`NewEnumerator0`
                (bind (_direction_2 _attacklefttime_2) (`Timeline|AttackRightTimeline` :!label _label_2)
                  (:`Update`
                    (`SceneComponent.K2_SetRelativeLocation` (`self.HitboxRight`) (`KismetMathLibrary.VLerp` (`self.HitboxPositionInactiveRight`) (`self.HitboxPositionActiveRight`) _attacklefttime_2) false false)
                    (`SceneComponent.SetRelativeScale3D` (`self.HitboxRight`) (`KismetMathLibrary.VLerp` (`self.HitboxLocalScaleInactive`) (`self.HitboxLocalScaleActive`) _attacklefttime_2)))
                  (:`Finished`
                    (switch `ETimelineDirection` _direction_2
                      (:`Forward`
                        (set `self.AttackStateRight` "NewEnumerator1"))
                      (:`Backward`
                        (set `self.AttackStateRight` "NewEnumerator2")
                        (`self.OnMeleeAttackFinishedRight`))))))
              (:`NewEnumerator1`
                (goto _label_2 :!via `Reverse`)))))))
    (:`then_1`
      (switch `/Game/Unicorn/Core/Engine/EGrowthState` (`self.ChargeGrowthState`)
        (:`NewEnumerator1`
          (bind (_direction_3 _growth) (`Timeline|ChargeTimeline` :!label _label_3)
            (:`Update`
              (`self.SetActorScale3D` (`KismetMathLibrary.VLerp` (`self.NormalSize`) (`self.ChargedSize`) _growth)))
            (:`Finished`
              (switch `ETimelineDirection` _direction_3
                (:`Forward`
                  (set `self.ChargeGrowthState` "NewEnumerator3")
                  (`self.SetBossState` "NewEnumerator2")
                  (`ResourceComponent.SetCurrentResource` _healthcomponent (`ResourceComponent.MaxResource` _healthcomponent))
                  (set `self.bDead` false))
                (:`Backward`
                  (set `self.ChargeGrowthState` "NewEnumerator0")
                  (`self.SetBossState` "NewEnumerator0"))))))
        (:`NewEnumerator2`
          (goto _label_3 :!via `Reverse`))))
    (:`then_2`
      (if (`self.bMovingToStationaryPosition`)
        (bind (_direction_4 _movementpercent) (`Timeline|MovementToSttationPos`)
          (:`Update`
            (bind _returnvalue_2 (`KismetMathLibrary.VLerp` (`self.StationStartPosition`) (`self.StationaryPosition`) _movementpercent))
            (`self.K2_TeleportTo` _returnvalue_2 (`KismetMathLibrary.FindLookAtRotation` _returnvalue_2 (`UnicornAIController.GetAimLocationOnActor` _returnvalue (`UnicornAIController.GetTargetActor` _returnvalue)))))
          (:`Finished`
            (set `self.bMovingToStationaryPosition` false)
            (`self.SetBossState` "NewEnumerator3")
            (bind _outactors (`GameplayStatics.GetAllActorsOfClass` "/Game/BP_GroundDamage.BP_GroundDamage_C"))
            (for _array_element _outactors
              (`/Game/BP_GroundDamage.FinishCharging` _array_element))))))))

(event `OnMeleeAttackFinishedLeft`
  (if (`|EnumEquality` (`self.AttackStateRight`) "NewEnumerator2")
    (`self.OnMeleeAttackFinished`)))

(event `OnMeleeAttackFinishedRight`
  (if (`|EnumEquality` (`self.AttackStateLeft`) "NewEnumerator2")
    (`self.OnMeleeAttackFinished`)))

(event `EventNotifyBeamFinished`
  (`self.NotifyBeamFinished`))

(event `self.DoMeleeAttack`
  (`self.DoRandomMeleeAttack`))

(event `self.DoRangedAttack`
  (`self.ShootIceSpike`))

(event `self.OnDeath`
  (switch `/Game/Unicorn/Core/Engine/EBossState` (`self.GetBossState`)
    (:`NewEnumerator0`
      ;[1 1 1] Check if power pillars remain
      (bind _outactors (`GameplayStatics.GetAllActorsOfClass` "/Game/Unicorn/Characters/UnicornCharacter/BP_PowerPIllor.BP_PowerPIllor_C"))
      (if (> (`KismetArrayLibrary.Array_Length` _outactors) 0)
        ;[1 1 1] If so, activate the pillar, change the body color, and change state to transitioning
        (`self.SetBossState` "NewEnumerator1")
        (`/Game/Unicorn/Characters/UnicornCharacter/BP_PowerPIllor.ActivatePillar` (`|GetArrayItem` _outactors) self)
        (`self.SetEnragedColor`)
        (`self.SetBossState` "NewEnumerator1")
        (else
          (`self.BecomeStationary`))))
    (:`NewEnumerator1`
      (`self.SetLifeSpan` 0.001))))

(fn `BecomeStationary`
  (`self.SetBossState` "NewEnumerator1")
  (`/Game/BP_DestructibleGround.DestroyGround` (`self.MiddleCeilingBlock`))
  (set `self.StationStartPosition` (`self.K2_GetActorLocation`))
  (set `self.bMovingToStationaryPosition` true)
  (bind _outactors (`GameplayStatics.GetAllActorsOfClass` "/Game/Unicorn/ObjectsForScenes/BP_Portal.BP_Portal_C"))
  (for _array_element _outactors
    (`self.K2_DestroyActor` _array_element))
  (`self.SetShield` false)
  (bind _outactors_2 (`GameplayStatics.GetAllActorsOfClass` "/Game/BP_GroundDamage.BP_GroundDamage_C"))
  (for _array_element_2 _outactors_2
    (`SceneComponent.SetVisibility` (`/Game/BP_GroundDamage.Cube` _array_element_2) true false))
  (return))

(fn `BeginGroundDamage`)

(fn `BeStunned`
  (params (StunPower :type "/Game/Unicorn/Core/Engine/EPowerLevel Enum" :default "NewEnumerator0"))
  (returns (Success :type Boolean))
  (return true))

(fn `ChargeBoss`
  (`MaterialInstanceDynamic.SetScalarParameterValue` (`self.BodyMat`) (`UnicornMaterialParameters.Emissive`) (`self.EnragedEmissive`))
  (set `self.ChargeGrowthState` "NewEnumerator1")
  (`self.SetShield` true)
  (return))

(fn `DechargeBoss`
  (`self.SetBossState` "NewEnumerator1")
  (`self.ResetColor`)
  (set `self.ChargeGrowthState` "NewEnumerator2")
  (return))

(fn `DoBeamAttack`
  (bind _returnvalue (`|SpawnActorFromClass` "/Game/Unicorn/Spells/BP_BossBeam.BP_BossBeam_C" (`KismetMathLibrary.MakeTransform` (`self.K2_GetActorLocation`)) "Undefined" "OverrideRootScale" null "TE_Player" "TE_PlayerEnemy" null))
  (add `/Game/Unicorn/Spells/BP_BossBeam.BeamFinished` _returnvalue (`|CreateDelegate` :!event `EventNotifyBeamFinished`))
  (return))

(fn `DoRandomMeleeAttack`
  (switch `int` (`KismetMathLibrary.RandomIntegerInRange` 0 2)
    (:`Default`
      (`self.MeleeAttack` "NewEnumerator0" :!label _label))
    (:`0`
      (`self.MeleeAttack` "NewEnumerator2"))
    (:`1`
      (`self.MeleeAttack` "NewEnumerator1"))
    (:`2`
      (goto _label)))
  (return))

(fn `GetBossCon`
  (returns (ReturnValue :type "/Game/Unicorn/Characters/UnicornCharacter/BP_CapsuleCon_Boss Object Reference"))
  (bind _asbp_capsule_con_boss (cast `/Game/Unicorn/Characters/UnicornCharacter/BP_CapsuleCon_Boss` (`AIBlueprintHelperLibrary.GetAIController` self)))
  (return _asbp_capsule_con_boss))

(fn `GetBossState`
  (returns (ReturnValue :type "/Game/Unicorn/Core/Engine/EBossState Enum"))
  (return (`/Game/Unicorn/Characters/UnicornCharacter/BP_CapsuleCon_Boss.GetBossState` (`self.GetBossCon`))))

(fn `HitActor`
  (params (HitActor :type "Actor Object Reference"))
  (if (`TeamComponent.IsSameTeam` (`self.TeamComponent`) HitActor)
    _
    (elif (not (`KismetArrayLibrary.Array_Contains` (`self.HitActors`) (`local.HitActor`)))
      (`KismetArrayLibrary.Array_Add` (`self.HitActors`) (`local.HitActor`))
      (message `HealthInterface.LoseHealth` (`local.HitActor`) (`self.MeleeDamage`))
      (return))))

(fn `Invincible`
  (returns (ReturnValue :type Boolean))
  (return (or (`self.ShieldIsActive`) (`|EnumEquality` (`self.GetBossState`) "NewEnumerator1") (`|EnumEquality` (`self.GetBossState`) "NewEnumerator2"))))

(fn `Knockback`
  (params (KnockbackOrigin :type "Vector Structure") (VelocityMagnitude :type "Float (double-precision)"))
  (returns (Success :type Boolean))
  (return true))

(fn `LoseHealth`
  (params (HealthLost :type "Float (double-precision)"))
  (returns (bDied :type Boolean) (ReturnValue :type Boolean))
  (if (`self.Invincible`)
    (return false true)
    (else
      (bind (_bdied _returnvalue) (`parent.LoseHealth` (`local.HealthLost`)))
      (return _bdied _returnvalue))))

(fn `MeleeAttack`
  (params (AttackType :type "/Game/Unicorn/Core/Engine/EHand Enum" :default "NewEnumerator0") (AttackTime :type "Float (double-precision)"))
  (`|SpawnActorFromClass` "/Game/Unicorn/Characters/UnicornCharacter/BT_BossAoE.BT_BossAoE_C" (`self.GetTransform`) "Undefined" "OverrideRootScale" null null)
  (`KismetSystemLibrary.K2_SetTimerDelegate` (`|CreateDelegate` :!event `OnMeleeAttackFinished`) (`self.MeleeAttackTime`))
  (return))

(fn `ResetColor`
  (set `self.bHurt` false)
  (`TimelineComponent.SetNewTime` (`self.HurtColorTimeline`) 0.0)
  (`MaterialInstanceDynamic.SetVectorParameterValue` (`self.BodyMat`) (`UnicornMaterialParameters.Color`) (`self.BodyColor`))
  (`MaterialInstanceDynamic.SetScalarParameterValue` (`self.BodyMat`) (`UnicornMaterialParameters.Emissive`) (`self.NormalEmissive`))
  (return))

(fn `SetBossState`
  (params (BossState :type "/Game/Unicorn/Core/Engine/EBossState Enum" :default "NewEnumerator0"))
  (`/Game/Unicorn/Characters/UnicornCharacter/BP_CapsuleCon_Boss.SetBossState` (`self.GetBossCon`) BossState)
  (return))

(fn `SetEnragedColor`
  (set `self.bHurt` false)
  (`TimelineComponent.SetNewTime` (`self.HurtColorTimeline`) 0.0)
  (`MaterialInstanceDynamic.SetVectorParameterValue` (`self.BodyMat`) (`UnicornMaterialParameters.Color`) (`self.HurtColor`))
  (return))

(fn `SetShield`
  (params (isActive :type Boolean))
  (if isActive
    (`SceneComponent.SetVisibility` (`self.Shield`) true false)
    (set `self.ShieldIsActive` true)
    (else
      (`SceneComponent.SetVisibility` (`self.Shield`) false false)
      (set `self.ShieldIsActive` false))))

(fn `ShootIceSpike`
  (bind _returnvalue (`self.GetCapsuleController`))
  (bind _returnvalue_2 (`SceneComponent.K2_GetComponentLocation` (`self.LeftEye`)))
  (`self.SetShield` false)
  (`|SpawnActorFromClass` "/Game/Unicorn/Spells/BP_IceSpike.BP_IceSpike_C" (`KismetMathLibrary.MakeTransform` _returnvalue_2 (`KismetMathLibrary.FindLookAtRotation` _returnvalue_2 (`UnicornAIController.GetAimLocationOnActor` _returnvalue (`UnicornAIController.GetTargetActor` _returnvalue)))) "Undefined" "OverrideRootScale" null 50.0 (1000.0 0.0 0.0) 3.0 (1.0 4.0 1.0) false 50.0 (0.0 0.0 0.0) 25.0 null false 5.0 (`self.Team`) "TE_PlayerEnemy" null)
  (`KismetSystemLibrary.K2_SetTimerDelegate` (`|CreateDelegate` :!event `OnRangedAttackFinished`) (`self.RangedAttackTime`))
  (return))

(fn `UserConstructionScript`
  (set `TeamComponent.Team` (`self.Team`) (`self.TeamComponent`))
  (bind _returnvalue (`KismetMaterialLibrary.CreateDynamicMaterialInstance` "/Game/Unicorn/Characters/UnicornCharacter/M_CapsuleMaterial.M_CapsuleMaterial"))
  (bind _output_get (set `self.BodyMat` _returnvalue))
  (`MaterialInstanceDynamic.SetVectorParameterValue` _output_get (`UnicornMaterialParameters.Color`) (`self.BodyColor`))
  (`PrimitiveComponent.SetMaterial` (`self.Sphere`) 0 (`self.BodyMat`))
  (`SceneComponent.SetRelativeScale3D` (`self.HitboxRight`) (`self.HitboxLocalScaleInactive`))
  (`SceneComponent.SetRelativeScale3D` (`self.HitboxLeft`) (`self.HitboxLocalScaleInactive`))
  (`SceneComponent.K2_SetRelativeLocation` (`self.HitboxRight`) (`self.HitboxPositionInactiveRight`) false false)
  (`SceneComponent.K2_SetRelativeLocation` (`self.HitboxLeft`) (`self.HitboxPositionInactiveLeft`) false false))