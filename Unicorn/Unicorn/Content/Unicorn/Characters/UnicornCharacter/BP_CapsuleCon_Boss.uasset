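; AI controller Blueprint for a prototype capsule boss that runs the BT_BossProto behavior tree on BeginPlay.
; It exposes SetBossState and GetBossState, which write and read an EBossState enum on the blackboard under the BossStateName key.
; Both accessors act only when the blackboard is valid, and Tick is disabled.
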(event `self.ReceiveBeginPlay`
  (`parent.ReceiveBeginPlay`)
  (`self.RunBehaviorTree` "/Game/Unicorn/Characters/UnicornCharacter/BT_BossProto.BT_BossProto"))

(fn `GetBossState`
  (returns (ReturnValue :type "/Game/Unicorn/Core/Engine/EBossState Enum"))
  (`/Engine/EditorBlueprintResources/StandardMacros.IsValid` (`self.Blackboard`)
    (:`Is Valid`
      (return (cast `/Game/Unicorn/Core/Engine/EBossState` (`BlackboardComponent.GetValueAsEnum` (`self.Blackboard`) (`self.BossStateName`)))))))

(fn `SetBossState`
  (params (BossState :type "/Game/Unicorn/Core/Engine/EBossState Enum" :default "NewEnumerator0"))
  (`/Engine/EditorBlueprintResources/StandardMacros.IsValid` (`self.Blackboard`)
    (:`Is Valid`
      (`BlackboardComponent.SetValueAsEnum` (`self.Blackboard`) (`self.BossStateName`) (`local.BossState`))
      (return))))

(fn `UserConstructionScript`
  (`parent.UserConstructionScript`))