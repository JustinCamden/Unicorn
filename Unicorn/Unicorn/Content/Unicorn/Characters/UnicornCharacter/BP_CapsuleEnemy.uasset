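; BP_CapsuleEnemy is an enemy character Blueprint with a team affiliation and a vision component.
; The construction script copies its Team variable into the TeamComponent, and BeginPlay prints that team as a debug string.
; GetVisionComponent returns the Vision component to callers.
; It has no other active logic, as the overlap and Tick events are empty.
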(event `self.ReceiveBeginPlay`
  (`KismetSystemLibrary.PrintString` (`|GetEnumeratorNameAsString` (`TeamComponent.Team` (`self.TeamComponent`)))))

(fn `GetVisionComponent`
  (returns (ReturnValue :type "SceneComponent Object Reference"))
  (return (`self.Vision`)))

(fn `UserConstructionScript`
  (set `TeamComponent.Team` (`self.Team`) (`self.TeamComponent`)))