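; Power pillar actor that opens on activation and charges the boss passed to it until destroyed.
; ActivatePillar stores the boss and sets a flag that Tick polls to play a timeline sliding Mid from Core toward Top.
; When opened, it activates a particle effect targeted from pillar to boss and calls ChargeBoss.
; DestroyPillar decharges the boss, spawns a BP_Portal at its location and removes itself via a tiny lifespan.
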(event `self.ReceiveBeginPlay`)

(event `self.ReceiveTick`
  (params (DeltaSeconds :type "Float (single-precision)"))
  (if (`self.bPillarOpening`)
    (bind (_direction _openpercent) (`Timeline|PillarOpeningTimeline`)
      (:`Update`
        (`SceneComponent.K2_SetRelativeLocation` (`self.Mid`) (`KismetMathLibrary.VLerp` (`SceneComponent.RelativeLocation` (`self.Core`)) (`SceneComponent.RelativeLocation` (`self.Top`)) _openpercent) false false))
      (:`Finished`
        (set `self.bPillarOpening` false)
        (set `self.bPillarActive` true)
        (`ActorComponent.Activate` (`self.ParticleSystem`) false)
        (`ParticleSystemComponent.SetActorParameter` (`self.ParticleSystem`) "SourceActor" self)
        (`ParticleSystemComponent.SetActorParameter` (`self.ParticleSystem`) "TargetActor" (`self.ActiveBoss`))
        (`/Game/Unicorn/Characters/UnicornCharacter/BP_BossProto.ChargeBoss` (`self.ActiveBoss`))))))

(fn `ActivatePillar`
  (params (Boss :type "/Game/Unicorn/Characters/UnicornCharacter/BP_BossProto Object Reference"))
  (set `self.ActiveBoss` Boss)
  (set `self.bPillarOpening` true)
  (return))

(fn `DestroyPillar`
  (`/Game/Unicorn/Characters/UnicornCharacter/BP_BossProto.DechargeBoss` (`self.ActiveBoss`))
  (`|SpawnActorFromClass` "/Game/Unicorn/ObjectsForScenes/BP_Portal.BP_Portal_C" (`KismetMathLibrary.MakeTransform` (`self.K2_GetActorLocation`)) "Undefined" "OverrideRootScale" null null)
  (`self.SetLifeSpan` 0.01)
  (return))

(fn `UserConstructionScript`)