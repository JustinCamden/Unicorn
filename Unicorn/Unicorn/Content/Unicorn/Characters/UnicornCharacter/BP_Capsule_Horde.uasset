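; BP_Capsule_Horde is a team-based capsule character that turns into a delayed explosion when it dies.
; Construction sets its team and tints the sphere through a dynamic material.
; On death it turns orange, makes its controller passive and starts a timer to explode.
; The explosion spawns effect and sound, sends damage to every other actor overlapping ExplosionCollision regardless of team, then removes itself via a tiny lifespan.
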(event `self.ReceiveBeginPlay`
  (`parent.ReceiveBeginPlay`))

(event `self.ReceiveTick`
  (params (DeltaSeconds :type "Float (single-precision)"))
  (`parent.ReceiveTick` DeltaSeconds))

(event `self.OnDeath`
  (`self.BeginExplosion`))

(fn `BeginExplosion`
  (`MaterialInstanceDynamic.SetVectorParameterValue` (`self.BodyMat`) (`UnicornMaterialParameters.Color`) (struct :`R` 1.0 :`G` 0.141186 :`A` 1.0))
  (set `self.bDead` true)
  (`UnicornAIController.SetIsPassive` (`self.GetCapsuleController`) true)
  (`KismetSystemLibrary.K2_SetTimer` null "Explode" (`self.ExplosionDeathTime`))
  (return))

(fn `Explode`
  (`|SpawnActorFromClass` "/Game/Unicorn/Spells/BP_Explosion.BP_Explosion_C" (`KismetMathLibrary.MakeTransform` (`SceneComponent.K2_GetComponentLocation` (`self.Mesh`)) (struct) (`self.ExplosionScale`)) "Undefined" "OverrideRootScale" null null)
  (`GameplayStatics.SpawnSoundAtLocation` "/Game/ProSoundCollection_v1_3/Magic_Spells/Cues/fireball_blast_projectile_spell_01_Cue.fireball_blast_projectile_spell_01_Cue" (`SceneComponent.K2_GetComponentLocation` (`self.Mesh`)) (struct) 1.0 1.0 0.0 "/Game/ATT_Spell.ATT_Spell" "/Game/CON_Spell.CON_Spell")
  (for _array_element (`PrimitiveComponent.GetOverlappingActors` (`self.ExplosionCollision`) null)
    (`/Engine/EditorBlueprintResources/StandardMacros.IsValid` _array_element
      (:`Is Valid`
        (if (!= _array_element self)
          (message `HealthInterface.LoseHealth` _array_element (`self.ExplosionDamage`))))))
  (`self.SetLifeSpan` 0.01)
  (return))

(fn `UserConstructionScript`
  (set `TeamComponent.Team` (`self.Team`) (`self.TeamComponent`))
  (bind _returnvalue (`KismetMaterialLibrary.CreateDynamicMaterialInstance` "/Game/Unicorn/Characters/UnicornCharacter/M_CapsuleMaterial.M_CapsuleMaterial"))
  (bind _output_get (set `self.BodyMat` _returnvalue))
  (`MaterialInstanceDynamic.SetVectorParameterValue` _output_get (`UnicornMaterialParameters.Color`) (`self.BodyColor`))
  (`PrimitiveComponent.SetMaterial` (`self.Sphere`) 0 (`self.BodyMat`)))