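; BP_CapsuleControl_Melee is the AI controller for the melee capsule enemy, running BT_Capsule_Melee on its controlled BP_Capsule_Melee pawn.
; On BeginPlay it binds to the pawn's melee-attack-finished notification.
; Each finished attack sets RecentlyCompletedMeleeAttack and restarts a one-shot timer that clears the flag after RecentlyAttackedTimerTime, provided that duration is above zero.
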(event `self.ReceiveBeginPlay`
  (`parent.ReceiveBeginPlay`)
  (bind _asbp_capsule_melee (cast `/Game/Unicorn/Characters/UnicornCharacter/BP_Capsule_Melee` (`self.K2_GetPawn`)))
  (add `/Game/Unicorn/Characters/UnicornCharacter/BP_Capsule_Melee.NotifyMeleeAttackFinished` _asbp_capsule_melee (`|CreateDelegate` :!event `OnMeleeAttackFinished`))
  (`self.RunBehaviorTree` "/Game/Unicorn/Characters/UnicornCharacter/BT_Capsule_Melee.BT_Capsule_Melee"))

(event `self.ReceiveTick`
  (params (DeltaSeconds :type "Float (single-precision)"))
  (`parent.ReceiveTick` DeltaSeconds))

(event `OnMeleeAttackFinished`
  (if (> (`self.RecentlyAttackedTimerTime`) 0.0)
    (`KismetSystemLibrary.K2_ClearAndInvalidateTimerHandle` (`self.RecentlyAttackedTimer`))
    (set `self.bRecentlyCompletedMeleeAttack` true)
    (bind _returnvalue (`KismetSystemLibrary.K2_SetTimerDelegate` (`|CreateDelegate` :!event `OnMeleeAttackTimerFinished`) (`self.RecentlyAttackedTimerTime`)))
    (set `self.RecentlyAttackedTimer` _returnvalue)))

(event `OnMeleeAttackTimerFinished`
  (set `self.bRecentlyCompletedMeleeAttack` false))

(fn `UserConstructionScript`
  (`parent.UserConstructionScript`))