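; Ranged capsule character that fires ice spikes at its controller's current target and can dash to a given location.
; Attacks spawn BP_IceSpike from the SpellLauncher, rotated toward the controller's aim point, tagged with the character's team.
; Dashes disable collision and gravity, raise emissive glow, and step via Teleport in Tick, with a timeout that snaps to the goal.
; Ending a dash restores state, flags RecentlyDashed temporarily and signals completion.
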(event `self.ReceiveBeginPlay`
  (`parent.ReceiveBeginPlay`))

(event `self.ReceiveTick`
  (params (DeltaSeconds :type "Float (single-precision)"))
  (`parent.ReceiveTick` DeltaSeconds)
  (`/Engine/EditorBlueprintResources/StandardMacros.IsValid` self
    (:`Is Valid`
      (if (`self.bDashing`)
        (if (<= (`KismetMathLibrary.VSize` (- (`self.DashGoal`) (`self.K2_GetActorLocation`))) (`self.DashTolerance`))
          (`KismetSystemLibrary.K2_ClearAndInvalidateTimerHandle` (`self.DashTimeoutTimer`))
          (`self.EndDash` true)
          (else
            (`self.K2_TeleportTo` (`KismetMathLibrary.VInterpTo_Constant` (`self.K2_GetActorLocation`) (`self.DashGoal`) (`GameplayStatics.GetWorldDeltaSeconds`) (`self.DashSpeed`)) (`self.K2_GetActorRotation`))))))))

(event `self.DoRangedAttack`
  (`self.ShootIceSpike`))

(event `RecentlyDashedTimerExpired`
  (set `self.bRecentlyDashed` false))

(event `DashTimeoutTimerFinished`
  (`self.K2_TeleportTo` (`self.DashGoal`) (`self.K2_GetActorRotation`))
  (`self.EndDash` false))

(fn `DashToLocation`
  (params (GoalLocation :type "Vector Structure"))
  (bind _capsulecomponent (`self.CapsuleComponent`))
  (set `self.DashGoal` (`KismetMathLibrary.MakeVector` GoalLocation_X GoalLocation_Y (+ GoalLocation_Z (`CapsuleComponent.CapsuleHalfHeight` (`self.CapsuleComponent`)))))
  (`MaterialInstanceDynamic.SetScalarParameterValue` (`self.BodyMat`) (`UnicornMaterialParameters.Emissive`) (`self.DashEmissive`))
  (`PrimitiveComponent.SetCollisionEnabled` (`self.Mesh`) "NoCollision")
  (`PrimitiveComponent.SetEnableGravity` _capsulecomponent false)
  (`PrimitiveComponent.SetCollisionEnabled` _capsulecomponent "NoCollision")
  (set `self.bDashing` true)
  (`KismetSystemLibrary.K2_ClearAndInvalidateTimerHandle` (`self.DashTimeoutTimer`))
  (bind _returnvalue (`KismetSystemLibrary.K2_SetTimerDelegate` (`|CreateDelegate` :!event `DashTimeoutTimerFinished`) (`self.DashTimeoutTime`)))
  (set `self.DashTimeoutTimer` _returnvalue)
  (`KismetSystemLibrary.K2_ClearAndInvalidateTimerHandle` (`self.RecentlyDashedTimer`))
  (`GameplayStatics.SpawnSoundAttached` "/Game/ProSoundCollection_v1_3/Magic_Spells/Cues/whoosh_magic_spell_02_Cue.whoosh_magic_spell_02_Cue" (`self.CapsuleComponent`) "None" (0.0 0.0 0.0) (struct) "KeepRelativeOffset" false 1.0 1.0 0.0 "/Game/ATT_Spell.ATT_Spell" "/Game/CON_Spell.CON_Spell")
  (return))

(fn `EndDash`
  (params (Success :type Boolean))
  (bind _capsulecomponent (`self.CapsuleComponent`))
  (`MaterialInstanceDynamic.SetScalarParameterValue` (`self.BodyMat`) (`UnicornMaterialParameters.Emissive`) 0.25)
  (`PrimitiveComponent.SetCollisionEnabled` (`self.Mesh`) "QueryOnly")
  (`PrimitiveComponent.SetEnableGravity` _capsulecomponent true)
  (`PrimitiveComponent.SetCollisionEnabled` _capsulecomponent "QueryAndPhysics")
  (set `self.bDashing` false)
  (`KismetSystemLibrary.K2_ClearAndInvalidateTimerHandle` (`self.DashTimeoutTimer`))
  (`KismetSystemLibrary.K2_SetTimerDelegate` (`|CreateDelegate` :!event `RecentlyDashedTimerExpired`) (`self.RecentlyDashedTime`))
  (set `self.bRecentlyDashed` true)
  (`self.DashCompleted`)
  (return))

(fn `ShootIceSpike`
  (bind _returnvalue (`self.GetCapsuleController`))
  (bind _returnvalue_2 (`SceneComponent.K2_GetComponentLocation` (`self.SpellLauncher`)))
  (`|SpawnActorFromClass` "/Game/Unicorn/Spells/BP_IceSpike.BP_IceSpike_C" (`KismetMathLibrary.MakeTransform` _returnvalue_2 (`KismetMathLibrary.FindLookAtRotation` _returnvalue_2 (`UnicornAIController.GetAimLocationOnActor` _returnvalue (`UnicornAIController.GetTargetActor` _returnvalue)))) "Undefined" "OverrideRootScale" null 50.0 (1000.0 0.0 0.0) 3.0 (1.0 4.0 1.0) false 50.0 (0.0 0.0 0.0) 25.0 null false 5.0 (`self.Team`) "TE_PlayerEnemy" null)
  (`KismetSystemLibrary.K2_SetTimerDelegate` (`|CreateDelegate` :!event `OnRangedAttackFinished`) (`self.RangedAttackTime`))
  (return))

(fn `UserConstructionScript`
  (`parent.UserConstructionScript`))