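; BP_DestructibleGround is a piece of ground that breaks apart when its DestroyGround function is called.
; DestroyGround turns on physics and gravity for the destructible component and applies damage at the actor's location with an upward impulse.
; It then hides the Cube, disables its collision and sets a lifespan so the actor removes itself.
; The event graph and construction script hold no logic.
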(event `self.ReceiveBeginPlay`)

(fn `DestroyGround`
  (bind (_returnvalue_x _returnvalue_y _returnvalue_z) (`KismetMathLibrary.BreakVector` (`self.K2_GetActorLocation`)))
  (bind _cube (`self.Cube`))
  (`PrimitiveComponent.SetSimulatePhysics` (`self.DestructibleComponent`) true)
  (`DestructibleComponent.ApplyDamage` (`self.DestructibleComponent`) 100.0 (`self.K2_GetActorLocation`) (`KismetMathLibrary.GetDirectionUnitVector` (`KismetMathLibrary.MakeVector` _returnvalue_x _returnvalue_y (- _returnvalue_z 100.0)) (`self.K2_GetActorLocation`)) 500.0)
  (`PrimitiveComponent.SetEnableGravity` (`self.DestructibleComponent`) true)
  (`self.SetLifeSpan` (`self.DestructionLifespan`))
  (`SceneComponent.SetVisibility` _cube false false)
  (`PrimitiveComponent.SetCollisionEnabled` _cube "NoCollision"))

(fn `UserConstructionScript`)