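; Ground area-of-effect marker actor, apparently for a damage zone, that shows when it has finished charging.
; The construction script gives its Cube a dynamic instance of M_AoEMaterial, stored as DamageMat.
; FinishCharging sets the Charged flag and switches the material's emissive scalar to ChargedEmissive.
; The event graph is empty, so charge timing and damage are not handled in these graphs.
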(fn `FinishCharging`
  (set `self.bCharged` true)
  (`MaterialInstanceDynamic.SetScalarParameterValue` (`self.DamageMat`) (`UnicornMaterialParameters.Emissive`) (`self.ChargedEmissive`))
  (return))

(fn `UserConstructionScript`
  (bind _returnvalue (`KismetMaterialLibrary.CreateDynamicMaterialInstance` "/Game/Unicorn/Characters/UnicornCharacter/M_AoEMaterial.M_AoEMaterial"))
  (bind _output_get (set `self.DamageMat` _returnvalue))
  (`PrimitiveComponent.SetMaterial` (`self.Cube`) 0 _output_get))